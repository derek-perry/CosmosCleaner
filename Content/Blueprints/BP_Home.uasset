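; BP_Home is the player's home location, with refuel and shop zones that open their menus when BP_Character walks in.
; Two box colliders ask the CosmosCleaner GameInstance to create the home widget in Refuel or Cargo mode and track a PlayerInside flag.
; A one-second start delay ignores initial overlaps, and DoOnce gates reset after a short delay to debounce repeat triggers.
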(event OnComponentBeginOverlap(BoxCollision_Shop)
  (params (OverlappedComponent :type Primitive%20Component%20Object%20Reference) (OtherActor :type Actor%20Object%20Reference) (OtherComp :type Primitive%20Component%20Object%20Reference) (OtherBodyIndex :type Integer) (bFromSweep :type Boolean) (SweepResult :type Hit%20Result%20Structure%20%28by%20ref%29))
  (bind _gameinstance (Variables|Default|GetGameInstance))
  ;[0.9583 0.9583 0.9583] Collider Check - Shop
  (Utilities|Casting|CastToBP_Character OtherActor)
  (Variables|Default|SetPlayerInside? true)
  (if (not (Variables|Default|GetStartDelay?))
    (Utilities|FlowControl|DoOnce false :!label _label
      (:Completed
        (Utilities|FlowControl|Sequence
          (:then_0
            (Default|WidgetCreateHome _gameinstance "Cargo")
            ;[0 1 0.25] DEBUG
            (Default|DebugPrint _gameinstance "Home-Shop Entered" "(R=0.058824,G=0.615686,B=0.192157,A=1.000000)" 2.0 self "None"))
          (:then_1
            (Utilities|FlowControl|Delay 0.1)
            (goto _label Reset)))))))

(event OnComponentEndOverlap(BoxCollision_Shop)
  (params (OverlappedComponent :type Primitive%20Component%20Object%20Reference) (OtherActor :type Actor%20Object%20Reference) (OtherComp :type Primitive%20Component%20Object%20Reference) (OtherBodyIndex :type Integer))
  ;[0.9583 0.9583 0.9583] Collider Check - Shop
  (Utilities|Casting|CastToBP_Character OtherActor)
  (Variables|Default|SetPlayerInside? false))

(event OnComponentBeginOverlap(BoxCollision_Fuel)
  (params (OverlappedComponent :type Primitive%20Component%20Object%20Reference) (OtherActor :type Actor%20Object%20Reference) (OtherComp :type Primitive%20Component%20Object%20Reference) (OtherBodyIndex :type Integer) (bFromSweep :type Boolean) (SweepResult :type Hit%20Result%20Structure%20%28by%20ref%29))
  (bind _gameinstance (Variables|Default|GetGameInstance))
  ;[0.9583 0.9583 0.9583] Collider Check - Fuel
  (Utilities|Casting|CastToBP_Character OtherActor)
  (Variables|Default|SetPlayerInside? true)
  (if (not (Variables|Default|GetStartDelay?))
    (Utilities|FlowControl|DoOnce false :!label _label
      (:Completed
        (Utilities|FlowControl|Sequence
          (:then_0
            (Default|WidgetCreateHome _gameinstance "Refuel")
            ;[0 1 0.25] DEBUG
            (Default|DebugPrint _gameinstance "Home-Fuel Entered" "(R=0.058824,G=0.615686,B=0.192157,A=1.000000)" 2.0 self "None"))
          (:then_1
            (Utilities|FlowControl|Delay 0.1)
            (goto _label Reset)))))))

(event OnComponentEndOverlap(BoxCollision_Fuel)
  (params (OverlappedComponent :type Primitive%20Component%20Object%20Reference) (OtherActor :type Actor%20Object%20Reference) (OtherComp :type Primitive%20Component%20Object%20Reference) (OtherBodyIndex :type Integer))
  ;[0.9583 0.9583 0.9583] Collider Check - Fuel
  (Utilities|Casting|CastToBP_Character OtherActor)
  (Variables|Default|SetPlayerInside? false))

(event EventBeginPlay
  ;[0 1 0] BeginPlay
  (Utilities|FlowControl|Sequence
    (:then_0
      ;[0.9583 0.9583 0.9583] Set Start Delay at Start for 1 Second
      (Variables|Default|SetStartDelay? true)
      (Utilities|FlowControl|Delay 1.0)
      (Variables|Default|SetStartDelay? false))
    (:then_1
      ;[0.9583 0.9583 0.9583] Get/Set GameInstance Ref
      (bind _ascosmos_cleaner_game_instance (Utilities|Casting|CastToCosmosCleaner_GameInstance (Game|GetGameInstance)))
      (Variables|Default|SetGameInstance _ascosmos_cleaner_game_instance))
    (:then_2
      ;[0 1 0.25] DEBUG
      (Default|DebugPrint (Variables|Default|GetGameInstance) "BP_Home Created" "(R=0.058824,G=0.615686,B=0.192157,A=1.000000)" 2.0 self ""))))

(fn ConstructionScript)