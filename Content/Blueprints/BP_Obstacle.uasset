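; BP_Obstacle is a destructible space-debris obstacle that drifts with a random Y/Z velocity impulse from BeginPlay.
; A dynamic material colors it red or green depending on whether its scale exceeds a size threshold.
; Projectile hits drain Health; on death it spawns an explosion, and large pieces also split into two half-scale copies of itself.
; Player-collision damage and the timeline that keeps it on the 2D plane are present but never run.
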(event Custom|SizeCheck
  ;[1 1 1] Check Obstacle Size
  (if (> (.z (.scale (Transformation|GetActorTransform self))) 0.75)
    (Rendering|Material|SetVectorParameterValue (Variables|Default|GetObstacleMeshMatDyn) "Color" "(R=0.291667,G=0.000000,B=0.000000,A=1.000000)" :!class /Script/Engine.MaterialInstanceDynamic)
    (else
      (Rendering|Material|SetVectorParameterValue (Variables|Default|GetObstacleMeshMatDyn) "Color" "(R=0.098786,G=0.291667,B=0.000000,A=1.000000)" :!class /Script/Engine.MaterialInstanceDynamic))))

(event EventBeginPlay
  (Utilities|FlowControl|Sequence
    (:then_0
      ;[1 1 1] CatcherAreaMesh Dynamic Material
      (Variables|Default|SetObstacleMeshMat (Rendering|Material|GetMaterial (Variables|Default|GetObstacleMesh) 0))
      (bind _returnvalue (Rendering|Material|CreateDynamicMaterialInstance (Variables|Default|GetObstacleMesh) 0 (Variables|Default|GetObstacleMeshMat) "ObstacleMeshMatDyn" :!class /Script/Engine.PrimitiveComponent))
      (Variables|Default|SetObstacleMeshMatDyn _returnvalue))
    (:then_1
      ;[1 1 1] Set Velocity
      (Physics|AddImpulse (Variables|Default|GetObstacleMesh) (Math|Vector|MakeVector 0.0 (Utilities|Select :Index (Math|Random|RandomIntegerinRange 0 1) :Option%200 (* (Math|Random|RandomFloatinRange -1.0 1.0) (Math|Random|RandomFloatinRange -2.5e+02 2.5e+02)) :Option%201 0.0) (Utilities|Select :Index (Math|Random|RandomIntegerinRange 0 1) :Option%200 (* (Math|Random|RandomFloatinRange -1.0 1.0) (Math|Random|RandomFloatinRange -2.5e+02 2.5e+02)) :Option%201 0.0)) "None" true))
    (:then_2
      ;[1 1 1] Check Obstacle Size
      (if (> (.z (.scale (Transformation|GetActorTransform self))) 0.75)
        (Rendering|Material|SetVectorParameterValue (Variables|Default|GetObstacleMeshMatDyn) "Color" "(R=0.291667,G=0.000000,B=0.000000,A=1.000000)" :!class /Script/Engine.MaterialInstanceDynamic)
        (else
          (Rendering|Material|SetVectorParameterValue (Variables|Default|GetObstacleMeshMatDyn) "Color" "(R=0.098786,G=0.291667,B=0.000000,A=1.000000)" :!class /Script/Engine.MaterialInstanceDynamic))))))

(event Collision|EventHit
  (params (MyComp :type Primitive%20Component%20Object%20Reference) (Other :type Actor%20Object%20Reference) (OtherComp :type Primitive%20Component%20Object%20Reference) (bSelfMoved :type Boolean) (HitLocation :type Vector :default "0, 0, 0") (HitNormal :type Vector :default "0, 0, 0") (NormalImpulse :type Vector :default "0, 0, 0") (Hit :type Hit%20Result%20Structure%20%28by%20ref%29))
  (bind _self self)
  (bind _self_2 self)
  (bind _returnvalue (Transformation|GetActorTransform _self))
  (bind _returnvalue_2 (Transformation|GetActorTransform _self_2))
  ;[1 1 1] OnHit with a certain actor, Take Health
  ;;[1 1 1] If Projectile Collsion
  (Utilities|Casting|CastToBP_Projectile Other)
  (Variables|Default|SetHealth (- (Variables|Default|GetHealth) 25.0))
  ;[1 1 1] Check if collision would kill this obstacle? If so, Kill Obstacle and determine whether to spawn smaller bits or just destroy
  (if (not (> (Variables|Default|GetHealth) 0.1))
    (if (> (.z (.scale (Transformation|GetActorTransform self))) 0.75)
      ;[1 1 1] Spawn Halfsize Space Bit
      (Game|SpawnActorfromClass "BP_Obstacle_C" (Math|Transform|MakeTransform (Math|Vector|MakeVector 0.0 (+ (.y (.location _returnvalue_2)) (Math|Random|RandomFloatinRange -1e+01 1e+01)) (+ (.z (.location _returnvalue_2)) (Math|Random|RandomFloatinRange -1e+01 1e+01))) (Math|Rotator|MakeRotator (Math|Random|RandomFloatinRange -3.6e+02 3.6e+02) (Math|Random|RandomFloatinRange -3.6e+02 3.6e+02) (Math|Random|RandomFloatinRange -3.6e+02 3.6e+02)) (Math|Vector|MakeVector (* (.x (.scale _returnvalue_2)) 0.5) (* (.y (.scale _returnvalue_2)) 0.5) (* (.z (.scale _returnvalue_2)) 0.5))) "AdjustIfPossibleButAlwaysSpawn" 0 0)
      ;[1 1 1] Spawn Halfsize Space Bit
      (Game|SpawnActorfromClass "BP_Obstacle_C" (Math|Transform|MakeTransform (Math|Vector|MakeVector 0.0 (+ (.y (.location _returnvalue)) (Math|Random|RandomFloatinRange -1e+01 1e+01)) (+ (.z (.location _returnvalue)) (Math|Random|RandomFloatinRange -1e+01 1e+01))) (Math|Rotator|MakeRotator (Math|Random|RandomFloatinRange -3.6e+02 3.6e+02) (Math|Random|RandomFloatinRange -3.6e+02 3.6e+02) (Math|Random|RandomFloatinRange -3.6e+02 3.6e+02)) (Math|Vector|MakeVector (* (.x (.scale _returnvalue)) 0.5) (* (.y (.scale _returnvalue)) 0.5) (* (.z (.scale _returnvalue)) 0.5))) "AdjustIfPossibleButAlwaysSpawn" 0 0)
      ;[1 1 1] Destroy
      (Game|SpawnActorfromClass "/Game/Blueprints/Blueprint_Effect_Explosion.Blueprint_Effect_Explosion_C" (Transformation|GetWorldTransform (Variables|Default|GetObstacleMesh)) "AdjustIfPossibleButAlwaysSpawn" 0 0)
      (Actor|DestroyActor)
      (else
        ;[1 1 1] Destroy
        (Game|SpawnActorfromClass "/Game/Blueprints/Blueprint_Effect_Explosion.Blueprint_Effect_Explosion_C" (Transformation|GetActorTransform self) "AdjustIfPossibleButAlwaysSpawn" 0 0)
        (Actor|DestroyActor)))))

(fn ConstructionScript)