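; Exhaust puff actor for the player's lander that shoots sideways, fades out and removes itself.
; On BeginPlay it gives its mesh a velocity-change impulse on world Y, opposite the lander's right vector Y component, scaled by BoostMultiplier.
; A timeline serves as a ticker, lowering a dynamic material's Opacity by a fixed step each update, so fade speed follows frame rate.
; The actor destroys itself once Opacity reaches zero.
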(event EventBeginPlay
  ;[1 1 1] Save Player
  (bind _asbp_player (Utilities|Casting|CastToBP_Player (Game|GetPlayerCharacter 0)))
  (bind _output_get (Variables|Default|SetPlayer _asbp_player))
  ;[1 1 1] Set Velocity
  (Physics|AddImpulse (Variables|Default|GetExhaustMesh) (Math|Vector|MakeVector 0.0 (* (* (.y (Math|Vector|GetRightVector (Variables|/Game/Blueprints/BP_Player.BP_Player_C|GetLander _output_get))) (Variables|Default|GetBoostMultiplier)) -1.0) 0.0) "None" true)
  ;[1 1 1] Setup Dynamic Material
  (Variables|Default|SetExhaustMat (Rendering|Material|GetMaterial (Variables|Default|GetExhaustMesh) 0))
  (bind _returnvalue (Rendering|Material|CreateDynamicMaterialInstance (Variables|Default|GetExhaustMesh) 0 (Variables|Default|GetExhaustMat) "ExhaustMatDyn" :!class /Script/Engine.PrimitiveComponent))
  (Variables|Default|SetExhaustMatDyn _returnvalue)
  (Utilities|FlowControl|Sequence
    (:then_0
      ;[1 1 1] Fade Opacity
      (Timeline|ExhaustTimeline Play
        (:Update
          (Utilities|FlowControl|Sequence
            (:then_0
              (bind _returnvalue_2 (Rendering|Material|GetScalarParameterValue (Variables|Default|GetExhaustMatDyn) "Opacity" :!class /Script/Engine.MaterialInstanceDynamic))
              (Rendering|Material|SetScalarParameterValue (Variables|Default|GetExhaustMatDyn) "Opacity" (- _returnvalue_2 0.02) :!class /Script/Engine.MaterialInstanceDynamic))
            (:then_1
              (bind _returnvalue_3 (Rendering|Material|GetScalarParameterValue (Variables|Default|GetExhaustMatDyn) "Opacity" :!class /Script/Engine.MaterialInstanceDynamic))
              (if (not (> _returnvalue_3 0.0))
                (Actor|DestroyActor)))))))))

(fn ConstructionScript)