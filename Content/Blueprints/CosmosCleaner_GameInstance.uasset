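; Game instance for Cosmos Cleaner that owns startup, saved settings and progress, music, and gameplay spawning.
; StartUp loads or creates the save, applies audio mixes and video settings, then opens splash and menu widgets or starts the game.
; StartGame spawns the ship matching its upgrade level, the homebase and HUD, and starts music.
; A delayed loop fills the world with weighted-random clutter built from saved cargo data, up to a maximum.
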(event Custom|InputModeGame
  (bind _returnvalue (Game|GetPlayerController 0))
  ;[1 0.8203 0] Set Input Mode to Game
  (Input|SetInputModeGameOnly _returnvalue false)
  (Variables|/Script/Engine.PlayerController|SetbEnableClickEvents _returnvalue false)
  (Variables|/Script/Engine.PlayerController|SetbEnableMouseOverEvents _returnvalue false)
  (Variables|/Script/Engine.PlayerController|SetbEnableTouchEvents _returnvalue false)
  (Variables|/Script/Engine.PlayerController|SetbEnableTouchOverEvents _returnvalue false)
  (Variables|/Script/Engine.PlayerController|SetbShowMouseCursor _returnvalue false)
  ;[0 1 0.25] DEBUG
  (CallFunction|DebugPrint (Utilities|String|Append "Input Mode Changed to Game using PC(" (Utilities|GetDisplayName _returnvalue) ")") "(R=0.058824,G=0.615686,B=0.192157,A=1.000000)" 2.0 0 "InputMode"))

(event Custom|DebugPrint
  (params (DebugText :type String) (TextColor :type Linear%20Color%20Structure) (Duration :type Float%20%28double-precision%29) (DebugActor :type Actor%20Object%20Reference) (Key :type Name))
  ;[0 1 0.25] DEBUG
  (Development|PrintString (Utilities|String|Append "[" (Utilities|GetDisplayName DebugActor) "] " DebugText) (Utilities|Struct|BreakStruct_SaveGame-Settings (Variables|SaveGame|GetStruct_SaveGame-Settings)) true TextColor Duration Key))

(event Custom|MusicStop
  (bind _sound_music_component (Variables|Audio|GetSound_Music-Component))
  ;[0.25 0 1] Stop Music
  (Utilities|IsValid _sound_music_component
    (:Is%20Valid
      (Audio|Components|Audio|Stop _sound_music_component)
      (Components|DestroyComponent _sound_music_component)
      ;[0 1 0.25] DEBUG
      (CallFunction|DebugPrint (Utilities|String|Append "Music Stopped (" (Utilities|GetDisplayName _sound_music_component) ")") "(R=0.058824,G=0.615686,B=0.192157,A=1.000000)" 2.0 0 "None"))))

(event Custom|AudioVolumeGetSet
  (bind _struct_savegame_settings (Variables|SaveGame|GetStruct_SaveGame-Settings))
  (bind (_audiomuted _audiosfx _audiomusic _audioambient) (Utilities|Struct|BreakStruct_SaveGame-Settings _struct_savegame_settings))
  ;[0.25 0 1] Get/Set Audio Volumes
  (if _audiomuted
    (Class|GameplayStatics|SetBaseSoundMix "/Game/Audio/A_Mix_Mute.A_Mix_Mute")
    (Audio|SetSoundMixClassOverride "/Game/Audio/A_Mix_Mute.A_Mix_Mute" "/Game/Audio/A_SoundClass_SFX.A_SoundClass_SFX" 1e-06 1.0 0.0 true)
    (Audio|SetSoundMixClassOverride "/Game/Audio/A_Mix_Mute.A_Mix_Mute" "/Game/Audio/A_SoundClass_Music.A_SoundClass_Music" 1e-06 1.0 0.0 true)
    (Audio|SetSoundMixClassOverride "/Game/Audio/A_Mix_Mute.A_Mix_Mute" "/Game/Audio/A_SoundClass_Ambient.A_SoundClass_Ambient" 1e-06 1.0 0.0 true)
    (else
      (Class|GameplayStatics|SetBaseSoundMix "/Game/Audio/A_Mix_Default.A_Mix_Default")
      (Audio|SetSoundMixClassOverride "/Game/Audio/A_Mix_Default.A_Mix_Default" "/Game/Audio/A_SoundClass_SFX.A_SoundClass_SFX" _audiosfx 1.0 0.0 true)
      (Audio|SetSoundMixClassOverride "/Game/Audio/A_Mix_Default.A_Mix_Default" "/Game/Audio/A_SoundClass_Music.A_SoundClass_Music" _audiomusic 1.0 0.0 true)
      (Audio|SetSoundMixClassOverride "/Game/Audio/A_Mix_Default.A_Mix_Default" "/Game/Audio/A_SoundClass_Ambient.A_SoundClass_Ambient" _audioambient 1.0 0.0 true))))

(event Custom|MusicPlay
  (params (SoundBase :type Sound%20Base%20Object%20Reference))
  ;[0.25 0 1] Play Music
  (Utilities|IsValid SoundBase
    (:Is%20Valid
      (Utilities|IsValid (Variables|Audio|GetSound_Music)
        (:Is%20Valid
          (if (not (== SoundBase (Variables|Audio|GetSound_Music)))
            (Utilities|FlowControl|Sequence :!label _label
              (:then_0
                (CallFunction|MusicStop))
              (:then_1
                (bind _output_get (Variables|Audio|SetSound_Music SoundBase))
                (bind _returnvalue (Audio|SpawnSound2D _output_get 1.0 1.0 0.0 0))
                (Variables|Audio|SetSound_Music-Component _returnvalue)))))
        (:Is%20Not%20Valid
          (goto _label))))))

(event Custom|SaveResetSettings
  (bind _savegamename (Variables|SaveGame|GetSaveGameName))
  ;[1 0.2462 0.3863] Reset SaveGame: Settings
  ;[0.9896 0.9896 0.9896] Reset Settings Struct in SaveGame
  (bind _returnvalue (SaveGame|LoadGamefromSlot _savegamename))
  (bind _assave_game_cosmos_cleaner (Utilities|Casting|CastToSaveGame_CosmosCleaner _returnvalue)
    (:then
      (Variables|/Game/Blueprints/SaveGame/SaveGame_CosmosCleaner.SaveGame_CosmosCleaner_C|SetSaveGame-Settings _assave_game_cosmos_cleaner (Variables|/Game/Blueprints/SaveGame/SaveGame_CosmosCleaner.SaveGame_CosmosCleaner_C|GetSaveGame-Settings_Default _assave_game_cosmos_cleaner))
      (Variables|SaveGame|SetStruct_SaveGame-Settings (Variables|/Game/Blueprints/SaveGame/SaveGame_CosmosCleaner.SaveGame_CosmosCleaner_C|GetSaveGame-Settings_Default _assave_game_cosmos_cleaner))
      ;[1 0.2462 0.3863] Save Game
      (SaveGame|SaveGametoSlot _assave_game_cosmos_cleaner _savegamename))
    (:CastFailed
      (CallFunction|SaveCurrent))))

(event Custom|SaveSettingsGetSet
  (bind _struct_savegame_settings (Variables|SaveGame|GetStruct_SaveGame-Settings))
  (bind (_videoframeratelimit _vsync_ _debug_) (Utilities|Struct|BreakStruct_SaveGame-Settings _struct_savegame_settings))
  ;[1 0.8203 0] Get/Set User Settings (Save/Apply FrameRateLimit and VSync)
  (bind _returnvalue (Settings|GetGameUserSettings))
  (Class|GameUserSettings|SetFrameRateLimit _returnvalue _videoframeratelimit)
  (Class|GameUserSettings|SetVSyncEnabled _returnvalue _vsync_)
  (Class|GameUserSettings|ApplySettings _returnvalue true)
  (Class|GameUserSettings|SaveSettings _returnvalue)
  ;[0 1 0.25] DEBUG
  (if _debug_
    (Development|ExecuteConsoleCommand "EnableAllScreenMessages" 0)
    (else
      (Development|ExecuteConsoleCommand "DisableAllScreenMessages" 0))))

(event Custom|SaveCurrent
  (bind _savegamename (Variables|SaveGame|GetSaveGameName))
  ;[1 0.2462 0.3863] Save Game with Current Values
  ;[0.9688 0.9688 0.9688] Check for existing savegame
  (bind _returnvalue (SaveGame|DoesSaveGameExist _savegamename))
  (if _returnvalue
    ;[0.9688 0.9688 0.9688] Load existing savegame
    (bind _returnvalue_2 (SaveGame|LoadGamefromSlot _savegamename))
    (bind _assave_game_cosmos_cleaner (Utilities|Casting|CastToSaveGame_CosmosCleaner _returnvalue_2)
      (:then
        (Variables|/Game/Blueprints/SaveGame/SaveGame_CosmosCleaner.SaveGame_CosmosCleaner_C|SetSaveGame-Settings _assave_game_cosmos_cleaner (Variables|SaveGame|GetStruct_SaveGame-Settings))
        (Variables|/Game/Blueprints/SaveGame/SaveGame_CosmosCleaner.SaveGame_CosmosCleaner_C|SetSaveGame-Game _assave_game_cosmos_cleaner (Variables|SaveGame|GetStruct_SaveGame-Game))
        ;[1 0.2462 0.3863] Save Game with Current Values
        (SaveGame|SaveGametoSlot _assave_game_cosmos_cleaner _savegamename))
      (:CastFailed
        ;[0.9688 0.9688 0.9688] Create new savegame
        (bind _returnvalue_3 (SaveGame|CreateSaveGameObject (Variables|SaveGame|GetSaveGameClass) :!label _label))
        (bind _assave_game_cosmos_cleaner_2 (Utilities|Casting|CastToSaveGame_CosmosCleaner _returnvalue_3))
        (Variables|/Game/Blueprints/SaveGame/SaveGame_CosmosCleaner.SaveGame_CosmosCleaner_C|SetSaveGame-Settings _assave_game_cosmos_cleaner_2 (Variables|SaveGame|GetStruct_SaveGame-Settings))
        (Variables|/Game/Blueprints/SaveGame/SaveGame_CosmosCleaner.SaveGame_CosmosCleaner_C|SetSaveGame-Game _assave_game_cosmos_cleaner_2 (Variables|SaveGame|GetStruct_SaveGame-Game))
        (SaveGame|SaveGametoSlot _assave_game_cosmos_cleaner_2 _savegamename)))
    (else
      (goto _label))))

(event Custom|SaveResetGame
  (bind _savegamename (Variables|SaveGame|GetSaveGameName))
  ;[1 0.2462 0.3863] Reset SaveGame: Game
  ;[0.9896 0.9896 0.9896] Reset Game Struct in SaveGame
  (bind _returnvalue (SaveGame|LoadGamefromSlot _savegamename))
  (bind _assave_game_cosmos_cleaner (Utilities|Casting|CastToSaveGame_CosmosCleaner _returnvalue)
    (:then
      (Variables|/Game/Blueprints/SaveGame/SaveGame_CosmosCleaner.SaveGame_CosmosCleaner_C|SetSaveGame-Game _assave_game_cosmos_cleaner (Variables|/Game/Blueprints/SaveGame/SaveGame_CosmosCleaner.SaveGame_CosmosCleaner_C|GetSaveGame-Game_Default _assave_game_cosmos_cleaner))
      (Variables|SaveGame|SetStruct_SaveGame-Game (Variables|/Game/Blueprints/SaveGame/SaveGame_CosmosCleaner.SaveGame_CosmosCleaner_C|GetSaveGame-Game_Default _assave_game_cosmos_cleaner))
      ;[1 0.2462 0.3863] Save Game
      (SaveGame|SaveGametoSlot _assave_game_cosmos_cleaner _savegamename))
    (:CastFailed
      (CallFunction|SaveCurrent))))

(event Custom|StartUp
  (params (MenuOrGame? :type Boolean))
  (bind _savegamename (Variables|SaveGame|GetSaveGameName))
  ;[0 1 0] Start Up Checks
  ;[0.9688 0.9688 0.9688] Check for existing savegame
  (bind _returnvalue (SaveGame|DoesSaveGameExist _savegamename))
  (if _returnvalue
    ;[0.9688 0.9688 0.9688] Load existing savegame
    (bind _returnvalue_2 (SaveGame|LoadGamefromSlot _savegamename))
    (bind _assave_game_cosmos_cleaner (Utilities|Casting|CastToSaveGame_CosmosCleaner _returnvalue_2)
      (:then
        (Variables|SaveGame|SetStruct_SaveGame-Game (Variables|/Game/Blueprints/SaveGame/SaveGame_CosmosCleaner.SaveGame_CosmosCleaner_C|GetSaveGame-Game _assave_game_cosmos_cleaner))
        (Variables|SaveGame|SetStruct_SaveGame-Settings (Variables|/Game/Blueprints/SaveGame/SaveGame_CosmosCleaner.SaveGame_CosmosCleaner_C|GetSaveGame-Settings _assave_game_cosmos_cleaner))
        ;[1 0.2462 0.3863] Save Game with Current Values
        (SaveGame|SaveGametoSlot _assave_game_cosmos_cleaner _savegamename)
        ;[0.25 0 1] Get/Set Audio Volumes
        (CallFunction|AudioVolumeGetSet)
        ;[1 0.8203 0] Get/Set User Settings (Save/Apply FrameRateLimit and VSync)
        (CallFunction|SaveSettingsGetSet)
        ;[0.974 0.974 0.974] Set NewPlayer? to False
        (Variables|SaveGame|SetNewPlayer? false)
        ;[0.974 0.974 0.974] Menu=True  or  Game=False
        (if MenuOrGame?
          ;[0.9792 0.9792 0.9792] False=Menu Start, True=Going to Menus from Game
          (if (Variables|In-Game|GetComingFromGame?)
            ;[0.8542 0.5278 0.3337] Create Widget - Existing Player Coming from In-Game: Main Menu
            (bind _returnvalue_3 (UserInterface|CreateWidget "/Game/Widgets/W_Menu-Main.W_Menu-Main_C"))
            (UserInterface|Viewport|AddtoViewport _returnvalue_3 0)
            (else
              ;[0.8542 0.5278 0.3337] Create Widget - Existing Player from Menu Start: Splash, then Main Menu
              (bind _returnvalue_4 (UserInterface|CreateWidget "/Game/Widgets/W_Splash.W_Splash_C"))
              (UserInterface|Viewport|AddtoViewport _returnvalue_4 0)
              (Variables|/Game/Widgets/W_Splash.W_Splash_C|SetNextWidget _returnvalue_4 "/Game/Widgets/W_Menu-Main.W_Menu-Main_C")))
          (else
            ;[0 1 0] Start Game
            (CallFunction|StartGame))))
      (:CastFailed
        ;[0.9688 0.9688 0.9688] Create new savegame
        (bind _returnvalue_5 (SaveGame|CreateSaveGameObject (Variables|SaveGame|GetSaveGameClass) :!label _label))
        (bind _assave_game_cosmos_cleaner_2 (Utilities|Casting|CastToSaveGame_CosmosCleaner _returnvalue_5))
        (Variables|SaveGame|SetStruct_SaveGame-Game (Variables|/Game/Blueprints/SaveGame/SaveGame_CosmosCleaner.SaveGame_CosmosCleaner_C|GetSaveGame-Game _assave_game_cosmos_cleaner_2))
        (Variables|SaveGame|SetStruct_SaveGame-Settings (Variables|/Game/Blueprints/SaveGame/SaveGame_CosmosCleaner.SaveGame_CosmosCleaner_C|GetSaveGame-Settings _assave_game_cosmos_cleaner_2))
        (SaveGame|SaveGametoSlot _assave_game_cosmos_cleaner_2 _savegamename)
        ;[0.25 0 1] Get/Set Audio Volumes
        (CallFunction|AudioVolumeGetSet)
        ;[1 0.8203 0] Get/Set User Settings (Save/Apply FrameRateLimit and VSync)
        (CallFunction|SaveSettingsGetSet)
        ;[0.974 0.974 0.974] Set NewPlayer? to True
        (Variables|SaveGame|SetNewPlayer? true)
        ;[0.974 0.974 0.974] Menu=True  or  Game=False
        (if MenuOrGame?
          ;[0.8542 0.5278 0.3337] Create Widget - First Play: Splash, then Menu-Settings, then Menu-Color, then Main Menu
          (bind _returnvalue_6 (UserInterface|CreateWidget "/Game/Widgets/W_Splash.W_Splash_C"))
          (UserInterface|Viewport|AddtoViewport _returnvalue_6 0)
          (Variables|/Game/Widgets/W_Splash.W_Splash_C|SetNextWidget _returnvalue_6 "/Game/Widgets/W_Menu-Settings.W_Menu-Settings_C")
          (else
            ;[0 1 0] Start Game
            (CallFunction|StartGame)))))
    (else
      (goto _label))))

(event Custom|StartGame
  ;[0 1 0] Start Game
  ;[1 0.8203 0] Set Input Mode to Game
  (CallFunction|InputModeGame)
  ;[0 1 0.7188] Spawn/Save Ref BP_CET (Player)
  (CallFunction|SpawnSaveRefCharacter)
  ;[0 1 0.7188] Spawn Max Amount of Clutter
  (CallFunction|SpawnClutterMax)
  ;[0 1 0.7188] Spawn/Save Ref BP_Homebase
  (CallFunction|SpawnSaveRefHomebase)
  ;[0.8542 0.5278 0.3337] Create Widget - HUD
  (CallFunction|WidgetCreateHUD)
  ;[0.25 0 1] Play Music : In-Game Music (A_Cue_Music_BrahmsTragicOvertureOp81)
  (CallFunction|MusicPlay "/Game/Audio/Music/A_Cue_Music_BrahmsTragicOvertureOp81.A_Cue_Music_BrahmsTragicOvertureOp81"))

(event Custom|SpawnSaveRefHomebase
  ;[0 1 0.7188] Save Ref/Spawn BP_Homebase
  (Utilities|IsValid (Variables|BPRefs|GetBP_HomeBase-ref)
    (:Is%20Valid
      (Actor|DestroyActor (Variables|BPRefs|GetBP_HomeBase-ref))
      (Variables|BPRefs|SetBP_HomeBase-ref 0))
    (:Is%20Not%20Valid
      (bind _outactors (Actor|GetAllActorsOfClass "/Game/Blueprints/BP_HomeBase.BP_HomeBase_C"))
      (for _array_element _outactors
        (Variables|BPRefs|SetBP_HomeBase-ref _array_element)
        ;[0 1 0.25] DEBUG
        (CallFunction|DebugPrint (Utilities|String|Append "BP_Homebase Ref Saved (" (Utilities|GetDisplayName (Variables|BPRefs|GetBP_HomeBase-ref)) ")") "(R=0.058824,G=0.615686,B=0.192157,A=1.000000)" 2.0 0 "None"))
      (Utilities|IsValid (Variables|BPRefs|GetBP_HomeBase-ref)
        (:Is%20Not%20Valid
          _))))
  (bind _returnvalue (Game|SpawnActorfromClass "/Game/Blueprints/BP_HomeBase.BP_HomeBase_C" (Math|Transform|MakeTransform "0, 0, 0" "0, 0, 0" "1.000000,1.000000,1.000000") "Undefined" "MultiplyWithRoot" 0 0))
  (Variables|BPRefs|SetBP_HomeBase-ref _returnvalue)
  ;[0 1 0.25] DEBUG
  (CallFunction|DebugPrint (Utilities|String|Append "BP_Homebase Spawned (" (Utilities|GetDisplayName (Variables|BPRefs|GetBP_HomeBase-ref)) ")") "(R=0.058824,G=0.615686,B=0.192157,A=1.000000)" 2.0 0 "None"))

(event Custom|SpawnSaveRefCharacter
  (bind _struct_savegame_game (Variables|SaveGame|GetStruct_SaveGame-Game))
  (bind _upgradelevel_ship (Utilities|Struct|BreakStruct_SaveGame-Game _struct_savegame_game))
  ;[0 1 0.7188] Save Ref/Spawn BP_Character (Player's Ship)
  (Utilities|IsValid (Variables|BPRefs|GetBP_Character-ref)
    (:Is%20Valid
      (Actor|DestroyActor (Variables|BPRefs|GetBP_Character-ref))
      (Variables|BPRefs|SetBP_Character-ref 0 :!label _label))
    (:Is%20Not%20Valid
      (bind _asbp_character (Utilities|Casting|CastToBP_Character (Game|GetPlayerCharacter 0))
        (:then
          (Actor|DestroyActor _asbp_character)
          (goto _label))
        (:CastFailed
          _))))
  (if (<= _upgradelevel_ship 1)
    (bind _returnvalue (Game|SpawnActorfromClass "/Game/Blueprints/BP_Character/BP_Character-Level1.BP_Character-Level1_C" (Math|Transform|MakeTransform "0.000000,0.000000,70.000000" "0, 0, 0" "1.000000,1.000000,1.000000") "Undefined" "MultiplyWithRoot" 0 0))
    (Variables|BPRefs|SetBP_Character-ref _returnvalue)
    (elif (== _upgradelevel_ship 2)
      (bind _returnvalue_2 (Game|SpawnActorfromClass "/Game/Blueprints/BP_Character/BP_Character-Level2.BP_Character-Level2_C" (Math|Transform|MakeTransform "0.000000,0.000000,70.000000" "0, 0, 0" "1.000000,1.000000,1.000000") "Undefined" "MultiplyWithRoot" 0 0))
      (Variables|BPRefs|SetBP_Character-ref _returnvalue_2)
      (else
        (if (== _upgradelevel_ship 3)
          _
          (else
            _))
        (bind _returnvalue_3 (Game|SpawnActorfromClass "/Game/Blueprints/BP_Character/BP_Character-Level3.BP_Character-Level3_C" (Math|Transform|MakeTransform "0.000000,0.000000,70.000000" "0, 0, 0" "1.000000,1.000000,1.000000") "Undefined" "MultiplyWithRoot" 0 0))
        (Variables|BPRefs|SetBP_Character-ref _returnvalue_3))))
  ;[0 1 0.25] DEBUG
  (CallFunction|DebugPrint (Utilities|String|Append "BP_Char Spawned/Ref Saved (" (Utilities|GetDisplayName (Variables|BPRefs|GetBP_Character-ref)) ")") "(R=0.058824,G=0.615686,B=0.192157,A=1.000000)" 2.0 0 "None"))

(event Custom|SpawnClutterMax
  ;[0 1 0.7188] Spawn Max Amount of Clutter
  (if (< (Variables|In-Game|GetClutterAmount) (Variables|In-Game|GetClutterAmountMax))
    (CallFunction|SpawnClutter)))

(event Custom|SpawnClutter
  (bind _bp_character_ref (Variables|BPRefs|GetBP_Character-ref))
  ;[0 1 0.7188] Spawn Clutter
  (if (< (Variables|In-Game|GetClutterAmount) (Variables|In-Game|GetClutterAmountMax)) :!label _label
    (Utilities|IsValid _bp_character_ref
      (:Is%20Valid
        (if (not (<= (.z (Transformation|GetActorLocation _bp_character_ref)) 2e+02))
          (Utilities|MacroClutterSpawn0 0 9)
          (Utilities|MacroClutterSpawn)
          (Math|Integer|IncrementInt (Variables|In-Game|GetClutterAmount)
            (:%20%20
              (Utilities|FlowControl|Delay 0.01)
              (goto _label))))))))

(event Custom|WidgetCreateHomebase
  ;[0.8542 0.5278 0.3337] Create Widget - Homebase
  (bind _returnvalue (UserInterface|CreateWidget "/Game/Widgets/W_HomeBase.W_HomeBase_C"))
  (bind _output_get (Variables|Widgets|SetW_Homebase _returnvalue))
  (UserInterface|Viewport|AddtoViewport _output_get 0)
  (Default|CollectingStop (Variables|BPRefs|GetBP_Character-ref))
  ;[0 1 0.25] DEBUG
  (CallFunction|DebugPrint (Utilities|String|Append "Homebase Widget Created (" (Utilities|GetDisplayName _output_get) ")") "(R=0.058824,G=0.615686,B=0.192157,A=1.000000)" 2.0 0 "None"))

(event Custom|WidgetCreateSettings
  (params (NextWidget :type User%20Widget%20Class%20Reference))
  ;[0.8542 0.5278 0.3337] Create Widget - Settings
  (bind _returnvalue (UserInterface|CreateWidget "/Game/Widgets/W_Menu-Settings.W_Menu-Settings_C"))
  (bind _output_get (Variables|Widgets|SetW_Settings _returnvalue))
  (UserInterface|Viewport|AddtoViewport _output_get 0)
  (Variables|/Game/Widgets/W_Menu-Settings.W_Menu-Settings_C|SetNextWidget _output_get NextWidget)
  ;[0 1 0.25] DEBUG
  (CallFunction|DebugPrint (Utilities|String|Append "Settings Widget Created (" (Utilities|GetDisplayName _output_get) ")") "(R=0.058824,G=0.615686,B=0.192157,A=1.000000)" 2.0 0 "None"))

(event Custom|WidgetCreateHUD
  ;[0.8542 0.5278 0.3337] Create Widget - HUD
  (bind _returnvalue (UserInterface|CreateWidget "/Game/Widgets/W_HUD.W_HUD_C"))
  (bind _output_get (Variables|Widgets|SetW_HUD _returnvalue))
  (UserInterface|Viewport|AddtoViewport _output_get 0)
  ;[0 1 0.25] DEBUG
  (CallFunction|DebugPrint (Utilities|String|Append "HUD Widget Created (" (Utilities|GetDisplayName _output_get) ")") "(R=0.058824,G=0.615686,B=0.192157,A=1.000000)" 2.0 0 "None"))