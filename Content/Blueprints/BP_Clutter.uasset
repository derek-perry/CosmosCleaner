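; Collectible clutter actor for Cosmos Cleaner, configured from ClutterData with mesh, dynamic-material color and randomized scale, drift and spin.
; While tractored, Tick applies distance-scaled impulses toward the character's tractor point; escaping restores rotation and reapplies stored impulses.
; Collection adds weight and type count to saved cargo if capacity allows, then destruction has the GameInstance replenish clutter.
; The color update also hides or destroys clutter outside the X-axis play band.
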(fn ConstructionScript
  (bind _clutterdata (Variables|Default|GetClutterData))
  (bind _color (Utilities|Struct|BreakStruct_SaveGame-Game-Cargo-Clutter _clutterdata))
  ;[0 1 0] Construct
  ;[0.9792 0.9792 0.9792] Get/Set Dynamic Material
  (Variables|Components|SetMaterial (Rendering|Material|GetMaterial (Variables|Components|GetMesh) 0))
  (bind _returnvalue (Rendering|Material|CreateDynamicMaterialInstance (Variables|Components|GetMesh) 0 (Variables|Components|GetMaterial) "MaterialDynamic" :!class /Script/Engine.PrimitiveComponent))
  (Variables|Components|SetMaterialDynamic _returnvalue)
  ;[0.9844 0.9844 0.9844] Check is savegame color is not empty/default
  (if (Class|KismetMathLibrary|LinearColorIsNearEqual _color "(R=0.000000,G=0.000000,B=0.000000,A=0.000000)" 0.0001)
    ;[0.9792 0.9792 0.9792] Change Color of Clutter to white
    (Rendering|Material|SetVectorParameterValue (Variables|Components|GetMaterialDynamic) "Color" "(R=1.000000,G=1.000000,B=1.000000,A=1.000000)" :!class /Script/Engine.MaterialInstanceDynamic)
    (else
      ;[0.9792 0.9792 0.9792] Change Color of Clutter to savegame color
      (Rendering|Material|SetVectorParameterValue (Variables|Components|GetMaterialDynamic) "Color" _color :!class /Script/Engine.MaterialInstanceDynamic))))

(event Custom|ClutterCollect
  (bind _clutterdata (Variables|Default|GetClutterData))
  (bind _gameinstance (Variables|Default|GetGameInstance))
  (bind (_type _weight) (Utilities|Struct|BreakStruct_SaveGame-Game-Cargo-Clutter _clutterdata))
  (bind _struct_savegame_game (Variables|/Game/Blueprints/CosmosCleaner_GameInstance.CosmosCleaner_GameInstance_C|GetStruct_SaveGame-Game _gameinstance))
  (bind (_cargo _cargoweight _cargoweightmax) (Utilities|Struct|BreakStruct_SaveGame-Game _struct_savegame_game))
  ;[1 0 0] Collect This Clutter
  ;[0.9531 0.9531 0.9531] Add this Clutter's Weight to Cargo Weight
  (if (<= _cargoweight (- _cargoweightmax _weight))
    (Utilities|Struct|SetmembersinStruct_SaveGame-Game _struct_savegame_game (+ _cargoweight _weight))
    ;[0.9583 0.9583 0.9583] Increment Inventory Count of specific clutter type
    (for _array_element (Utilities|Struct|BreakStruct_SaveGame-Game-Cargo _cargo)
      (if (Utilities|Enum|Equal(Enum) (.Type (Utilities|Struct|BreakStruct_SaveGame-Game-Cargo-Clutter _array_element)) _type)
        (bind _result (Math|Integer|IncrementInt (.Amount (Utilities|Struct|BreakStruct_SaveGame-Game-Cargo-Clutter _array_element)))
          (:%20%20
            (Default|NotifcationSpawn (Variables|/Game/Blueprints/CosmosCleaner_GameInstance.CosmosCleaner_GameInstance_C|GetW_HUD _gameinstance) (Utilities|Text|ToText(String) (Utilities|String|Append "+1 " (.Type (Utilities|Struct|BreakStruct_SaveGame-Game-Cargo-Clutter _array_element)) " 
" (Utilities|String|ToString(Integer) _result))))
            ;[1 0.2462 0.3863] Save Game with Current Values
            (Default|SaveCurrentValues _gameinstance)
            ;[1 0 0] Destroy This Clutter
            (CallFunction|ClutterDestroy)))))
    (Default|SaveCurrentValues _gameinstance))
  (CallFunction|ClutterDestroy))

(event Custom|ClutterDestroy
  (bind _gameinstance (Variables|Default|GetGameInstance))
  ;[1 0 0] Destroy This Clutter
  ;[1 0 0] Destroy Actor
  (Actor|DestroyActor)
  ;[0.9531 0.9531 0.9531] Decrement ClutterAmount
  (Math|Integer|DecrementInt (Variables|/Game/Blueprints/CosmosCleaner_GameInstance.CosmosCleaner_GameInstance_C|GetClutterAmount _gameinstance)
    (:%20%20
      (Default|SpawnClutterMax _gameinstance)
      ;[0 1 0.25] DEBUG
      (Default|DebugPrint _gameinstance "Clutter Bordered" "(R=0.058824,G=0.615686,B=0.192157,A=1.000000)" 2.0 self "ClutterBordered"))))

(event EventBeginPlay
  ;[0 1 0] BeginPlay
  ;[0.9583 0.9583 0.9583] Get/Set GameInstance Ref
  (bind _ascosmos_cleaner_game_instance (Utilities|Casting|CastToCosmosCleaner_GameInstance (Game|GetGameInstance)))
  (bind _output_get (Variables|Default|SetGameInstance _ascosmos_cleaner_game_instance))
  ;[0 1 0.25] DEBUG
  (Default|DebugPrint _output_get (Utilities|String|Append "Clutter Created" " (" (Utilities|String|ToString(Integer) (Variables|/Game/Blueprints/CosmosCleaner_GameInstance.CosmosCleaner_GameInstance_C|GetClutterAmount _output_get)) "/" (Utilities|String|ToString(Integer) (- (Variables|/Game/Blueprints/CosmosCleaner_GameInstance.CosmosCleaner_GameInstance_C|GetClutterAmountMax _output_get) 1)) ")") "(R=0.058824,G=0.615686,B=0.192157,A=1.000000)" 2.0 self "ClutterCreated"))

(event EventTick
  (params (DeltaSeconds :type Float%20%28single-precision%29))
  (bind _gameinstance (Variables|Default|GetGameInstance))
  (bind _mesh (Variables|Components|GetMesh))
  (bind _returnvalue (Transformation|GetWorldLocation _mesh))
  (bind _bp_character_ref (Variables|/Game/Blueprints/CosmosCleaner_GameInstance.CosmosCleaner_GameInstance_C|GetBP_Character-ref _gameinstance))
  (bind _scene_tractorpoint (Variables|/Game/Blueprints/BP_Character/BP_Character.BP_Character_C|GetScene_TractorPoint _bp_character_ref))
  (bind _returnvalue_2 (Transformation|GetWorldLocation _scene_tractorpoint))
  ;[0 1 0] Event Tick
  ;[0.9635 0.9635 0.9635] If tractoring? = true, then start tractoring toward character
  (if (Variables|Default|GetTractoring?)
    ;[0.974 0.974 0.974] Set Velocity to push clutter toward character
    (Physics|AddImpulse (Variables|Components|GetMesh) (Math|Vector|MakeVector (* (- (.x _returnvalue_2) (.x _returnvalue)) 0.15) (* (- (.y _returnvalue_2) (.y _returnvalue)) 0.15) (* (- (.z _returnvalue_2) (.z _returnvalue)) 0.15)) "None" true)))

(event Custom|ClutterTractorEnter
  ;[0.9792 0.9792 0.9792] Clutter Tractor Enter Actions
  ;[0.9479 0.9479 0.9479] Do the proper order of tractor setup
  (Variables|Default|SetRotationBeforeFaceChar (Transformation|GetActorRotation))
  (CallFunction|ClutterResetVelocity)
  (Variables|Default|SetTractoring? true))

(event Custom|ClutterTractorEscape
  ;[0.9792 0.9792 0.9792] Clutter Tractor Escape Actions
  ;[0.9479 0.9479 0.9479] Do the proper order of tractor escape
  (Variables|Default|SetTractoring? false)
  (Transformation|SetActorRotation (Variables|Default|GetRotationBeforeFaceChar) true)
  (CallFunction|ClutterSetVelocityInitial))

(event Custom|ClutterSetInitialScale
  (bind _clutterdata (Variables|Default|GetClutterData))
  (bind _initialscalevariation (Utilities|Struct|BreakStruct_SaveGame-Game-Cargo-Clutter _clutterdata))
  (bind (_x _y _z) (Math|Vector|BreakVector _initialscalevariation))
  (bind _returnvalue (Math|Random|RandomFloatinRange 1.0 _x))
  (bind _returnvalue_2 (Math|Random|RandomFloatinRange 1.0 _y))
  (bind _returnvalue_3 (Math|Random|RandomFloatinRange 1.0 _z))
  ;[0.9792 0.9792 0.9792] ClutterSetInitialScale
  ;[0.9375 0.9375 0.9375] Get/Set Initial Scale of Clutter (Variation within range)
  (if (Class|KismetMathLibrary|NotEqualExactlyVectorVector _initialscalevariation "0, 0, 0")
    (Transformation|SetActorScale3D self (Math|Vector|MakeVector _returnvalue _returnvalue_2 _returnvalue_3))
    (Variables|InitialValues|SetInitial_Scale (Math|Vector|MakeVector _returnvalue _returnvalue_2 _returnvalue_3))
    (else
      (Transformation|SetActorScale3D self "1.000000,1.000000,1.000000"))))

(event Custom|ClutterResetVelocity
  (bind _mesh (Variables|Components|GetMesh))
  ;[0.9792 0.9792 0.9792] Reset Clutter Velocity to 0
  ;[0.974 0.974 0.974] Reset both linear and angular velocity
  (Physics|SetPhysicsLinearVelocity _mesh "0, 0, 0" false "None")
  (Class|PrimitiveComponent|SetPhysicsAngularVelocityinDegrees _mesh "0, 0, 0" false "None"))

(event Custom|ClutterSetScaleInitial
  ;[0.9792 0.9792 0.9792] Reset Scale to Initial
  ;[0.9375 0.9375 0.9375] Get/Set Initial Scale of Clutter (Variation within range)
  (Transformation|SetActorScale3D self (Variables|InitialValues|GetInitial_Scale)))

(event Custom|ClutterSetVelocityInitial
  ;[0.9792 0.9792 0.9792] Reset Velocity to Initial
  ;[0.974 0.974 0.974] Set Initial Velocity
  (Physics|AddImpulse (Variables|Components|GetMesh) (Variables|InitialValues|GetInitial_Impulse) "None" true)
  (Class|PrimitiveComponent|AddAngularImpulseinDegrees (Variables|Components|GetMesh) (Variables|InitialValues|GetInitial_ImpulseAngular) "None" true))

(event Custom|ClutterSetInitialVelocity
  (bind _clutterdata (Variables|Default|GetClutterData))
  (bind (_initialvelocityroll _initialvelocityy _initialvelocityz) (Utilities|Struct|BreakStruct_SaveGame-Game-Cargo-Clutter _clutterdata))
  (bind _returnvalue (* _initialvelocityz -1.0))
  (bind _returnvalue_2 (* _initialvelocityy -1.0))
  (bind _returnvalue_3 (* _initialvelocityroll -1.0))
  (bind _returnvalue_4 (Math|Random|RandomFloatinRange _returnvalue_3 _initialvelocityroll))
  (bind _returnvalue_5 (Math|Random|RandomFloatinRange _returnvalue_2 _initialvelocityy))
  (bind _returnvalue_6 (Math|Random|RandomFloatinRange _returnvalue _initialvelocityz))
  ;[0.9792 0.9792 0.9792] ClutterSetInitialVelocity
  ;[0.974 0.974 0.974] Set Initial Velocity
  (Physics|AddImpulse (Variables|Components|GetMesh) (Math|Vector|MakeVector 0.0 _returnvalue_5 _returnvalue_6) "None" true)
  (Class|PrimitiveComponent|AddAngularImpulseinDegrees (Variables|Components|GetMesh) (Math|Vector|MakeVector _returnvalue_4 0.0 0.0) "None" true)
  (Variables|InitialValues|SetInitial_Impulse (Math|Vector|MakeVector 0.0 _returnvalue_5 _returnvalue_6))
  (Variables|InitialValues|SetInitial_ImpulseAngular (Math|Vector|MakeVector _returnvalue_4 0.0 0.0)))

(event Custom|ClutterChangeColor
  (params (Color :type Linear%20Color%20Structure :default "(R=0.000000,G=0.000000,B=0.000000,A=0.000000)"))
  ;[0.9792 0.9792 0.9792] Change/Check Color for Change
  ;[0.9844 0.9844 0.9844] Check is input color is not empty/default
  (if (Class|KismetMathLibrary|LinearColorIsNearEqual Color "(R=0.000000,G=0.000000,B=0.000000,A=0.000000)" 0.0001)
    ;[0.9792 0.9792 0.9792] Change Color of Clutter to savegame color
    (Rendering|Material|SetVectorParameterValue (Variables|Components|GetMaterialDynamic) "Color" (Utilities|Struct|BreakStruct_SaveGame-Game-Cargo-Clutter (Variables|Default|GetClutterData)) :!class /Script/Engine.MaterialInstanceDynamic)
    (else
      ;[0.9792 0.9792 0.9792] Change Color of Clutter to input color
      (Rendering|Material|SetVectorParameterValue (Variables|Components|GetMaterialDynamic) "Color" Color :!class /Script/Engine.MaterialInstanceDynamic)))
  ;[0.9583 0.9583 0.9583] Within play area/along x-axis? (Front to Back/Camera View) If out of range, destroy. If within certain range (but outside normal area), change color to barely opaque.
  (if (not (Math|Float|InRange(Float) (.x (Transformation|GetWorldLocation (Variables|Components|GetMesh))) -5e+01 5e+01))
    (if (Math|Float|InRange(Float) (.x (Transformation|GetWorldLocation (Variables|Components|GetMesh))) -2.5e+02 2.5e+02)
      (Rendering|Material|SetVectorParameterValue (Variables|Components|GetMaterialDynamic) "Color" "(R=0.000000,G=0.000000,B=0.000000,A=0.000000)" :!class /Script/Engine.MaterialInstanceDynamic)
      (else
        (Actor|DestroyActor)))))

(event Custom|ClutterCheckMat
  ;[0.9792 0.9792 0.9792] Check Mat for Change
  ;[0.9844 0.9844 0.9844] Check is savegame material is not empty
  (if (not (== (Utilities|Struct|BreakStruct_SaveGame-Game-Cargo-Clutter (Variables|Default|GetClutterData)) 0))
    ;[0.9792 0.9792 0.9792] Set mesh material based on savegame material
    (Rendering|Material|SetMaterial (Variables|Components|GetMesh) 0 0)))

(event Custom|ClutterSetup
  (bind _clutterdata (Variables|Default|GetClutterData))
  (bind (_type _id _value _weight _icon _mesh _material _color _initialvelocityroll _initialvelocityy _initialvelocityz _initialscalevariation _amount) (Utilities|Struct|BreakStruct_SaveGame-Game-Cargo-Clutter _clutterdata))
  ;[0 1 0] Clutter Setup Mesh, Mat, Color, Velocity, Scale, etc...
  ;[0.9479 0.9479 0.9479] Reset Velocity and Set to Saved Velocity
  (CallFunction|ClutterResetVelocity)
  ;[0.9792 0.9792 0.9792] ClutterSetInitialScale
  (CallFunction|ClutterSetInitialScale)
  ;[0.9792 0.9792 0.9792] ClutterSetInitialVelocity
  (CallFunction|ClutterSetInitialVelocity)
  ;[0.9792 0.9792 0.9792] Check Mesh for Change
  (CallFunction|ClutterCheckMesh)
  ;[0.9792 0.9792 0.9792] Check Mat for Change
  (CallFunction|ClutterCheckMat)
  ;[0.9792 0.9792 0.9792] Change/Check Color for Change
  (CallFunction|ClutterChangeColor "(R=0.000000,G=0.000000,B=0.000000,A=0.000000)")
  ;[0 1 0.25] DEBUG
  (Default|DebugPrint (Variables|Default|GetGameInstance) (Utilities|String|Append "ClutterCreated=" _type "," (Utilities|String|ToString(Integer) _id) "," (Utilities|String|ToString(Integer) _color) "," (Utilities|String|ToString(Integer) _amount)) "(R=0.058824,G=0.615686,B=0.192157,A=1.000000)" 2.0 self "ClutterCreated"))

(event Custom|ClutterCheckMesh
  (bind _clutterdata (Variables|Default|GetClutterData))
  (bind _mesh (Utilities|Struct|BreakStruct_SaveGame-Game-Cargo-Clutter _clutterdata))
  ;[0.9792 0.9792 0.9792] Check Mesh for Change
  ;[0.9844 0.9844 0.9844] Check is savegame mesh is not empty
  (if (not (== _mesh 0))
    ;[0.9792 0.9792 0.9792] Set mesh based on savegame mesh
    (Components|StaticMesh|SetStaticMesh (Variables|Components|GetMesh) _mesh)))