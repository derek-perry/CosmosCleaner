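; Menu player controller for CosmosCleaner that lets the pause input control the settings widget.
; On BeginPlay it adds the IMC_InGame Enhanced Input mapping context.
; IA_Pause gets the settings widget from the game instance, hides all its menus if open or otherwise calls its BatmanSettings function, then plays a click sound.
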(event Input|EnhancedActionEvents|EnhancedInputActionIA_Pause
  (params (ActionValue :type Boolean) (ElapsedSeconds :type Float%20%28double-precision%29) (TriggeredSeconds :type Float%20%28double-precision%29) (InputAction :type Input%20Action%20Object%20Reference :default "/Game/Input/IA_Pause.IA_Pause"))
  ;[0 0 0] Press Pause Button
  (:Started
    ;[0.974 0.974 0.974] Existing W_Settings?
    (bind _ascosmos_cleaner_game_instance (Utilities|Casting|CastToCosmosCleaner_GameInstance (Game|GetGameInstance)))
    (Utilities|IsValid (Variables|/Game/Blueprints/CosmosCleaner_GameInstance.CosmosCleaner_GameInstance_C|GetW_Settings _ascosmos_cleaner_game_instance)
      (:Is%20Valid
        ;[0.9688 0.9688 0.9688] Check for Open Settings Menu
        (if (Variables|/Game/Widgets/W_Menu-Settings.W_Menu-Settings_C|GetMenuOpen? (Variables|/Game/Blueprints/CosmosCleaner_GameInstance.CosmosCleaner_GameInstance_C|GetW_Settings _ascosmos_cleaner_game_instance))
          (Default|MenuHideAll (Variables|/Game/Blueprints/CosmosCleaner_GameInstance.CosmosCleaner_GameInstance_C|GetW_Settings _ascosmos_cleaner_game_instance))
          (else
            ;[1 0 0] Batman the Settings Widget
            (Default|BatmanSettings (Variables|/Game/Blueprints/CosmosCleaner_GameInstance.CosmosCleaner_GameInstance_C|GetW_Settings _ascosmos_cleaner_game_instance))))
        ;[0.25 0 1] Play Sound : Click
        (Audio|PlaySound2D "/Game/Audio/SFX/A_Cue_SFX_Click.A_Cue_SFX_Click" 1.0 1.0 0.0 0 0)))))

(event EventBeginPlay
  (bind _returnvalue (PlayerController|LocalPlayerSubsystems|GetEnhancedInputLocalPlayerSubsystem))
  ;[0 1 0] Begin Play
  ;[0 0 0] Input - Add IMC_InGame
  (Utilities|IsValid _returnvalue
    (:Is%20Valid
      (Input|AddMappingContext _returnvalue "/Game/Input/IMC_InGame.IMC_InGame" 0 "(bIgnoreAllPressedKeysUntilRelease=True,bForceImmediately=False,bNotifyUserSettings=False)"))))

(fn ConstructionScript)