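; BP_CargoDeposit is a goal zone that marks when the player is in position to deposit cargo.
; On BeginPlay it caches the player character as a BP_Player reference.
; GoalCollider overlap events set that player's IsCargoDepositing flag on entry and clear it on exit, ignoring actors that are not BP_Player.
; The deposit itself is not handled in this Blueprint, which only toggles the flag.
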(event OnComponentBeginOverlap(GoalCollider)
  (params (OverlappedComponent :type Primitive%20Component%20Object%20Reference) (OtherActor :type Actor%20Object%20Reference) (OtherComp :type Primitive%20Component%20Object%20Reference) (OtherBodyIndex :type Integer) (bFromSweep :type Boolean) (SweepResult :type Hit%20Result%20Structure%20%28by%20ref%29))
  ;[1 1 1] Goal Collider Checking
  (Utilities|Casting|CastToBP_Player OtherActor)
  (Variables|/Game/Blueprints/BP_Player.BP_Player_C|SetisCargoDepositing? (Variables|Default|GetPlayer) true))

(event OnComponentEndOverlap(GoalCollider)
  (params (OverlappedComponent :type Primitive%20Component%20Object%20Reference) (OtherActor :type Actor%20Object%20Reference) (OtherComp :type Primitive%20Component%20Object%20Reference) (OtherBodyIndex :type Integer))
  ;[1 1 1] Goal Collider Checking
  (Utilities|Casting|CastToBP_Player OtherActor)
  (Variables|/Game/Blueprints/BP_Player.BP_Player_C|SetisCargoDepositing? (Variables|Default|GetPlayer) false))

(event EventBeginPlay
  ;[1 1 1] Begin Play
  (Utilities|FlowControl|Sequence
    (:then_1
      ;[1 1 1] Save Player
      (bind _asbp_player (Utilities|Casting|CastToBP_Player (Game|GetPlayerCharacter 0)))
      (Variables|Default|SetPlayer _asbp_player))))

(fn ConstructionScript)