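; Player character for Cosmos Cleaner: flies with physics thrusters and gathers BP_Clutter through toggled tractor and collect overlap volumes.
; Thrust applies impulses along the up vector; roll uses angular impulses or, in mouse-movement mode, a timeline facing the cursor or touch.
; Thrusting drains GameInstance fuel and optional boost, saving each time and spawning exhaust; boost regenerates through a self-calling delay.
; Running out of fuel empties cargo, refuels and starts a new day.
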(event EventBeginPlay
  ;[0 1 0] BeginPlay
  ;[0.9635 0.9635 0.9635] Reset Velocity
  (Variables|/Script/Engine.MovementComponent|SetVelocity (Variables|Character|GetCharacterMovement) "0, 0, 0")
  ;[0.9635 0.9635 0.9635] Get/Set GameInstance Ref
  (bind _ascosmos_cleaner_game_instance (Utilities|Casting|CastToCosmosCleaner_GameInstance (Game|GetGameInstance)))
  (bind _output_get (Variables|Default|SetGameInstance _ascosmos_cleaner_game_instance))
  ;[0 1 0.25] DEBUG
  (Default|DebugPrint _output_get "Player Created" "(R=0.058824,G=0.615686,B=0.192157,A=1.000000)" 2.0 self "None")
  ;[0.9531 0.9531 0.9531] Set Camera's Arm Length based on Scroll Input
  (Variables|/Script/Engine.SpringArmComponent|SetTargetArmLength (Variables|Default|GetSpringArm_Camera) (Variables|/Game/Blueprints/CosmosCleaner_GameInstance.CosmosCleaner_GameInstance_C|GetCameraScrollLength _output_get))
  ;[0.9635 0.9635 0.9635] Reset Collecting Area
  (CallFunction|CollectingStop)
  ;[0.9688 0.9688 0.9688] Start: Regenerate Boost Over Time
  (CallFunction|BoostRegenStart))

(fn ConstructionScript)

(event OnComponentBeginOverlap(Mesh_TractorArea)
  (params (OverlappedComponent :type Primitive%20Component%20Object%20Reference) (OtherActor :type Actor%20Object%20Reference) (OtherComp :type Primitive%20Component%20Object%20Reference) (OtherBodyIndex :type Integer) (bFromSweep :type Boolean) (SweepResult :type Hit%20Result%20Structure%20%28by%20ref%29))
  ;[0.9792 0.9792 0.9792] Collider Check - Tractor Area
  (bind _asbp_clutter (Utilities|Casting|CastToBP_Clutter OtherActor))
  ;[0.9531 0.9531 0.9531] Clutter Tractor Enter Actions
  (Default|ClutterTractorEnter _asbp_clutter)
  ;[0 1 0.25] DEBUG
  (Default|DebugPrint (Variables|Default|GetGameInstance) "Clutter Tractor Enter" "(R=0.058824,G=0.615686,B=0.192157,A=1.000000)" 2.0 self "ClutterTractorEnter"))

(event OnComponentEndOverlap(Mesh_TractorArea)
  (params (OverlappedComponent :type Primitive%20Component%20Object%20Reference) (OtherActor :type Actor%20Object%20Reference) (OtherComp :type Primitive%20Component%20Object%20Reference) (OtherBodyIndex :type Integer))
  ;[0.9792 0.9792 0.9792] Collider Check - Tractor Area
  (bind _asbp_clutter (Utilities|Casting|CastToBP_Clutter OtherActor))
  ;[0.9531 0.9531 0.9531] Clutter Tractor Escape Actions
  (Default|ClutterTractorEscape _asbp_clutter)
  ;[0 1 0.25] DEBUG
  (Default|DebugPrint (Variables|Default|GetGameInstance) "Clutter Escaped Tractor Area" "(R=0.058824,G=0.615686,B=0.192157,A=1.000000)" 2.0 self "ClutterEscapedTractor"))

(event OnComponentBeginOverlap(Mesh_CollectArea)
  (params (OverlappedComponent :type Primitive%20Component%20Object%20Reference) (OtherActor :type Actor%20Object%20Reference) (OtherComp :type Primitive%20Component%20Object%20Reference) (OtherBodyIndex :type Integer) (bFromSweep :type Boolean) (SweepResult :type Hit%20Result%20Structure%20%28by%20ref%29))
  ;[0.9792 0.9792 0.9792] Collider Check - Collect Area
  (bind _asbp_clutter (Utilities|Casting|CastToBP_Clutter OtherActor))
  ;[1 0 0] Collect then Destroy the Clutter Collected
  (Default|ClutterCollect _asbp_clutter)
  ;[0 1 0.25] DEBUG
  (Default|DebugPrint (Variables|Default|GetGameInstance) "Clutter Collected" "(R=0.058824,G=0.615686,B=0.192157,A=1.000000)" 2.0 self "ClutterCollected"))

(event OnComponentEndOverlap(Mesh_CollectArea)
  (params (OverlappedComponent :type Primitive%20Component%20Object%20Reference) (OtherActor :type Actor%20Object%20Reference) (OtherComp :type Primitive%20Component%20Object%20Reference) (OtherBodyIndex :type Integer))
  ;[0.9792 0.9792 0.9792] Collider Check - Collect Area
  (Utilities|Casting|CastToBP_Clutter OtherActor)
  ;[0 1 0.25] DEBUG
  (Default|DebugPrint (Variables|Default|GetGameInstance) "Clutter Escaped Collect Area" "(R=0.058824,G=0.615686,B=0.192157,A=1.000000)" 2.0 self "ClutterEscapedCollect"))

(event Custom|CollectingStop
  (bind _mesh_collectarea (Variables|Default|GetMesh_CollectArea))
  ;[0 0 0] Collect
  ;[0.974 0.974 0.974] Set isCollecting? and Show/Hide CollectArea
  (Development|SetHiddeninGame _mesh_collectarea true true)
  (Collision|SetCollisionEnabled _mesh_collectarea "NoCollision")
  ;[0.974 0.974 0.974] Set isCollecting? to False
  (Variables|Default|SetisCollecting? false)
  ;[0 1 0.25] DEBUG
  (Default|DebugPrint (Variables|Default|GetGameInstance) "Collection Stopped" "(R=0.058824,G=0.615686,B=0.192157,A=1.000000)" 2.0 self "CollectionStopped"))

(event Custom|CollectingStart
  (bind _mesh_collectarea (Variables|Default|GetMesh_CollectArea))
  ;[0 0 0] Collect
  ;[0.974 0.974 0.974] Show/Hide CollectArea & TractorArea
  (Development|SetHiddeninGame _mesh_collectarea false true)
  (Collision|SetCollisionEnabled _mesh_collectarea "QueryOnly")
  ;[0.974 0.974 0.974] Set isCollecting? to True
  (Variables|Default|SetisCollecting? true)
  ;[0 1 0.25] DEBUG
  (Default|DebugPrint (Variables|Default|GetGameInstance) "Collection Started" "(R=0.058824,G=0.615686,B=0.192157,A=1.000000)" 2.0 self "CollectionStarted"))

(event Input|EnhancedActionEvents|EnhancedInputActionIA_Collect
  (params (ActionValue :type Boolean) (ElapsedSeconds :type Float%20%28double-precision%29) (TriggeredSeconds :type Float%20%28double-precision%29) (InputAction :type Input%20Action%20Object%20Reference :default "/Game/Input/IA_Collect.IA_Collect"))
  (bind _mesh_collectarea (Variables|Default|GetMesh_CollectArea))
  (bind _mesh_collectarea_2 (Variables|Default|GetMesh_CollectArea))
  ;[0 0 0] Collect
  (:Started
    ;[0.974 0.974 0.974] Show/Hide CollectArea & TractorArea
    (Development|SetHiddeninGame _mesh_collectarea_2 false true)
    (Collision|SetCollisionEnabled _mesh_collectarea_2 "QueryOnly")
    ;[0.974 0.974 0.974] Set isCollecting? to True
    (Variables|Default|SetisCollecting? true)
    ;[0 1 0.25] DEBUG
    (Default|DebugPrint (Variables|Default|GetGameInstance) "Collection Started" "(R=0.058824,G=0.615686,B=0.192157,A=1.000000)" 2.0 self "CollectionStarted"))
  (:Completed
    ;[0.974 0.974 0.974] Set isCollecting? and Show/Hide CollectArea
    (Development|SetHiddeninGame _mesh_collectarea true true)
    (Collision|SetCollisionEnabled _mesh_collectarea "NoCollision")
    ;[0.974 0.974 0.974] Set isCollecting? to False
    (Variables|Default|SetisCollecting? false)
    ;[0 1 0.25] DEBUG
    (Default|DebugPrint (Variables|Default|GetGameInstance) "Collection Stopped" "(R=0.058824,G=0.615686,B=0.192157,A=1.000000)" 2.0 self "CollectionStopped")))

(event Custom|RollStop
  (bind _returnvalue (Game|GetPlayerController 0))
  (bind _returnvalue_2 (Transformation|GetActorLocation))
  (bind _screenposition (Class|GameplayStatics|ProjectWorldtoScreen _returnvalue _returnvalue_2 false))
  (bind (_locationx _locationy _returnvalue_3) (Game|Player|GetMousePosition _returnvalue))
  (bind (_locationx_2 _locationy_2 _biscurrentlypressed) (Class|PlayerController|GetInputTouchState _returnvalue "Touch1"))
  (bind _returnvalue_4 (Math|Rotator|FindLookatRotation (Math|Vector|MakeVector (.x _screenposition) (.y _screenposition) 0.0) (Math|Vector|MakeVector _locationx_2 _locationy_2 0.0)))
  (bind _returnvalue_5 (Math|Rotator|FindLookatRotation (Math|Vector|MakeVector (.x _screenposition) (.y _screenposition) 0.0) (Math|Vector|MakeVector _locationx _locationy 0.0)))
  (bind _yaw (Math|Rotator|BreakRotator _returnvalue_5))
  (bind _yaw_2 (Math|Rotator|BreakRotator _returnvalue_4))
  (bind _returnvalue_6 (+ _yaw_2 9e+01))
  (bind _returnvalue_7 (+ _yaw 9e+01))
  ;[1 0 0.2812] Roll
  (Timeline|Timeline_Roll Stop
    (:Update
      (if _returnvalue_3
        (Transformation|SetActorRotation (Math|Rotator|MakeRotator _returnvalue_7 0.0 0.0))
        ;[0 1 0.25] DEBUG
        (Default|DebugPrint (Variables|Default|GetGameInstance) (Utilities|String|Append "RollLR-Mouse (" (Utilities|String|ToString(Float) _returnvalue_7) ")") "(R=0.058824,G=0.615686,B=0.192157,A=1.000000)" 1.0 self "RollLR")
        (elif _biscurrentlypressed
          (Transformation|SetActorRotation (Math|Rotator|MakeRotator _returnvalue_6 0.0 0.0))
          ;[0 1 0.25] DEBUG
          (Default|DebugPrint (Variables|Default|GetGameInstance) (Utilities|String|Append "RollLR-Touch (" (Utilities|String|ToString(Float) _returnvalue_6) ")") "(R=0.058824,G=0.615686,B=0.192157,A=1.000000)" 1.0 self "RollLR"))))))

(event Custom|BoostRegenStart
  (bind _gameinstance (Variables|Default|GetGameInstance))
  ;[0.9688 0.9688 0.9688] Regenerate Boost Over Time
  (if (< (Variables|/Game/Blueprints/CosmosCleaner_GameInstance.CosmosCleaner_GameInstance_C|GetBoost _gameinstance) 99.475)
    (Variables|/Game/Blueprints/CosmosCleaner_GameInstance.CosmosCleaner_GameInstance_C|SetBoost _gameinstance (+ (Variables|/Game/Blueprints/CosmosCleaner_GameInstance.CosmosCleaner_GameInstance_C|GetBoost _gameinstance) 0.525))
    (Utilities|FlowControl|Delay 0.01)
    (CallFunction|BoostRegenStart)
    (elif (< (Variables|/Game/Blueprints/CosmosCleaner_GameInstance.CosmosCleaner_GameInstance_C|GetBoost _gameinstance) 1e+02)
      (Variables|/Game/Blueprints/CosmosCleaner_GameInstance.CosmosCleaner_GameInstance_C|SetBoost _gameinstance 1e+02))))

(event Custom|RollStart
  (bind _returnvalue (Game|GetPlayerController 0))
  (bind _returnvalue_2 (Transformation|GetActorLocation))
  (bind _screenposition (Class|GameplayStatics|ProjectWorldtoScreen _returnvalue _returnvalue_2 false))
  (bind (_locationx _locationy _returnvalue_3) (Game|Player|GetMousePosition _returnvalue))
  (bind (_locationx_2 _locationy_2 _biscurrentlypressed) (Class|PlayerController|GetInputTouchState _returnvalue "Touch1"))
  (bind _returnvalue_4 (Math|Rotator|FindLookatRotation (Math|Vector|MakeVector (.x _screenposition) (.y _screenposition) 0.0) (Math|Vector|MakeVector _locationx_2 _locationy_2 0.0)))
  (bind _returnvalue_5 (Math|Rotator|FindLookatRotation (Math|Vector|MakeVector (.x _screenposition) (.y _screenposition) 0.0) (Math|Vector|MakeVector _locationx _locationy 0.0)))
  (bind _yaw (Math|Rotator|BreakRotator _returnvalue_5))
  (bind _yaw_2 (Math|Rotator|BreakRotator _returnvalue_4))
  (bind _returnvalue_6 (+ _yaw_2 9e+01))
  (bind _returnvalue_7 (+ _yaw 9e+01))
  ;[1 0 0.2812] Roll
  (Utilities|FlowControl|Sequence
    (:then_0
      (Timeline|Timeline_Roll SetNewTime
        (:Update
          (if _returnvalue_3
            (Transformation|SetActorRotation (Math|Rotator|MakeRotator _returnvalue_7 0.0 0.0))
            ;[0 1 0.25] DEBUG
            (Default|DebugPrint (Variables|Default|GetGameInstance) (Utilities|String|Append "RollLR-Mouse (" (Utilities|String|ToString(Float) _returnvalue_7) ")") "(R=0.058824,G=0.615686,B=0.192157,A=1.000000)" 1.0 self "RollLR")
            (elif _biscurrentlypressed
              (Transformation|SetActorRotation (Math|Rotator|MakeRotator _returnvalue_6 0.0 0.0))
              ;[0 1 0.25] DEBUG
              (Default|DebugPrint (Variables|Default|GetGameInstance) (Utilities|String|Append "RollLR-Touch (" (Utilities|String|ToString(Float) _returnvalue_6) ")") "(R=0.058824,G=0.615686,B=0.192157,A=1.000000)" 1.0 self "RollLR"))))))
    (:then_1
      (Timeline|Timeline_Roll PlayFromStart))))

(event Input|EnhancedActionEvents|EnhancedInputActionIA_Rotate
  (params (ActionValue :type Boolean) (ElapsedSeconds :type Float%20%28double-precision%29) (TriggeredSeconds :type Float%20%28double-precision%29) (InputAction :type Input%20Action%20Object%20Reference :default "/Game/Input/IA_Rotate.IA_Rotate"))
  (bind _returnvalue (Game|GetPlayerController 0))
  (bind _returnvalue_2 (Transformation|GetActorLocation))
  (bind _screenposition (Class|GameplayStatics|ProjectWorldtoScreen _returnvalue _returnvalue_2 false))
  (bind (_locationx _locationy _returnvalue_3) (Game|Player|GetMousePosition _returnvalue))
  (bind (_locationx_2 _locationy_2 _biscurrentlypressed) (Class|PlayerController|GetInputTouchState _returnvalue "Touch1"))
  (bind _returnvalue_4 (Math|Rotator|FindLookatRotation (Math|Vector|MakeVector (.x _screenposition) (.y _screenposition) 0.0) (Math|Vector|MakeVector _locationx_2 _locationy_2 0.0)))
  (bind _returnvalue_5 (Math|Rotator|FindLookatRotation (Math|Vector|MakeVector (.x _screenposition) (.y _screenposition) 0.0) (Math|Vector|MakeVector _locationx _locationy 0.0)))
  (bind _yaw (Math|Rotator|BreakRotator _returnvalue_5))
  (bind _yaw_2 (Math|Rotator|BreakRotator _returnvalue_4))
  (bind _returnvalue_6 (+ _yaw_2 9e+01))
  (bind _returnvalue_7 (+ _yaw 9e+01))
  ;[0 0 0] Press Move to Roll
  (:Triggered
    ;[0 1 0.25] DEBUG
    (Default|DebugPrint (Variables|Default|GetGameInstance) "RollGo" "(R=0.058824,G=0.615686,B=0.192157,A=1.000000)" 1.0 0 "RollLRTest"))
  (:Started
    ;[0.9583 0.9583 0.9583] Able to Roll?
    (if (Utilities|Struct|BreakStruct_SaveGame-Game (Variables|/Game/Blueprints/CosmosCleaner_GameInstance.CosmosCleaner_GameInstance_C|GetStruct_SaveGame-Game (Variables|Default|GetGameInstance)))
      ;[1 0 0.2812] Roll
      (Utilities|FlowControl|Sequence
        (:then_0
          (Timeline|Timeline_Roll SetNewTime
            (:Update
              (if _returnvalue_3
                (Transformation|SetActorRotation (Math|Rotator|MakeRotator _returnvalue_7 0.0 0.0))
                ;[0 1 0.25] DEBUG
                (Default|DebugPrint (Variables|Default|GetGameInstance) (Utilities|String|Append "RollLR-Mouse (" (Utilities|String|ToString(Float) _returnvalue_7) ")") "(R=0.058824,G=0.615686,B=0.192157,A=1.000000)" 1.0 self "RollLR")
                (elif _biscurrentlypressed
                  (Transformation|SetActorRotation (Math|Rotator|MakeRotator _returnvalue_6 0.0 0.0))
                  ;[0 1 0.25] DEBUG
                  (Default|DebugPrint (Variables|Default|GetGameInstance) (Utilities|String|Append "RollLR-Touch (" (Utilities|String|ToString(Float) _returnvalue_6) ")") "(R=0.058824,G=0.615686,B=0.192157,A=1.000000)" 1.0 self "RollLR"))))))
        (:then_1
          (Timeline|Timeline_Roll PlayFromStart)))))
  (:Completed
    (CallFunction|RollStop)))

(event Input|EnhancedActionEvents|EnhancedInputActionIA_ThrustY
  (params (ActionValue :type Float%20%28double-precision%29) (ElapsedSeconds :type Float%20%28double-precision%29) (TriggeredSeconds :type Float%20%28double-precision%29) (InputAction :type Input%20Action%20Object%20Reference :default "/Game/Input/IA_ThrustY.IA_ThrustY"))
  (bind _returnvalue (Math|Float|Clamp(Float) ActionValue -0.75))
  (bind _self self)
  (bind _self_2 self)
  (bind _gameinstance (Variables|Default|GetGameInstance))
  (bind _thrustermultiplier (Variables|MovementRate|GetThrusterMultiplier))
  (bind _thrustermultiplier_2 (Variables|MovementRate|GetThrusterMultiplier))
  (bind _boostthrustmultiplier (Variables|Boost|GetBoostThrustMultiplier))
  (bind _gameinstance_2 (Variables|Default|GetGameInstance))
  (bind _gameinstance_3 (Variables|Default|GetGameInstance))
  (bind _returnvalue_2 (Transformation|GetActorUpVector _self_2))
  (bind _returnvalue_3 (Transformation|GetActorUpVector _self))
  (bind _returnvalue_4 (* _returnvalue _thrustermultiplier))
  (bind _returnvalue_5 (* _returnvalue _thrustermultiplier_2 _boostthrustmultiplier))
  (bind _struct_savegame_game (Variables|/Game/Blueprints/CosmosCleaner_GameInstance.CosmosCleaner_GameInstance_C|GetStruct_SaveGame-Game _gameinstance))
  (bind _struct_savegame_game_2 (Variables|/Game/Blueprints/CosmosCleaner_GameInstance.CosmosCleaner_GameInstance_C|GetStruct_SaveGame-Game _gameinstance_3))
  ;[0 0 0] Press Up/Down to Thrust
  ;[0.9531 0.9531 0.9531] Able to Thrust?
  (if (!= _returnvalue 0.0)
    (if (> (Utilities|Struct|BreakStruct_SaveGame-Game (Variables|/Game/Blueprints/CosmosCleaner_GameInstance.CosmosCleaner_GameInstance_C|GetStruct_SaveGame-Game (Variables|Default|GetGameInstance))) 0.0)
      (if (Variables|Boost|GetBoosting?)
        (if (> (- (Variables|/Game/Blueprints/CosmosCleaner_GameInstance.CosmosCleaner_GameInstance_C|GetBoost (Variables|Default|GetGameInstance)) (Variables|Boost|GetBoostUDLossMultiplier)) 0.0)
          ;[1 0 0.2812] ThrustUD (Boosted)
          (Physics|AddImpulse (Variables|Collision|GetCapsuleComponent) (Math|Vector|MakeVector (* (.x _returnvalue_3) _returnvalue_5) (* (.y _returnvalue_3) _returnvalue_5) (* (.z _returnvalue_3) _returnvalue_5)) "None" false)
          ;[0 0.4141 1] Set Boost Amnt
          (Variables|/Game/Blueprints/CosmosCleaner_GameInstance.CosmosCleaner_GameInstance_C|SetBoost _gameinstance_2 (- (Variables|/Game/Blueprints/CosmosCleaner_GameInstance.CosmosCleaner_GameInstance_C|GetBoost _gameinstance_2) (Variables|Boost|GetBoostUDLossMultiplier)))
          ;[0.4062 1 0] Set Fuel Amnt
          (Utilities|Struct|SetmembersinStruct_SaveGame-Game _struct_savegame_game (- (Utilities|Struct|BreakStruct_SaveGame-Game _struct_savegame_game) (Variables|FuelLoss|GetFuelLossMultiplier)))
          ;[1 0.2462 0.3863] Save Game with Current Values
          (Default|SaveCurrent _gameinstance)
          ;[0 1 0.25] DEBUG
          (Default|DebugPrint (Variables|Default|GetGameInstance) (Utilities|String|Append "ThrustUD-Boosted (" (Utilities|String|ToString(Float) _returnvalue) ")") "(R=0.058824,G=0.615686,B=0.192157,A=1.000000)" 1.0 self "ThrustUD-Boosted")
          (else
            ;[1 0 0.2812] ThrustUD
            (Physics|AddImpulse (Variables|Collision|GetCapsuleComponent) (Math|Vector|MakeVector (* (.x _returnvalue_2) _returnvalue_4) (* (.y _returnvalue_2) _returnvalue_4) (* (.z _returnvalue_2) _returnvalue_4)) "None" false :!label _label)
            ;[0.4062 1 0] Set Fuel Amnt
            (Utilities|Struct|SetmembersinStruct_SaveGame-Game _struct_savegame_game_2 (- (Utilities|Struct|BreakStruct_SaveGame-Game _struct_savegame_game_2) (Variables|FuelLoss|GetFuelLossMultiplierLesser)))
            ;[1 0.2462 0.3863] Save Game with Current Values
            (Default|SaveCurrent _gameinstance_3)
            ;[0 1 0.25] DEBUG
            (Default|DebugPrint (Variables|Default|GetGameInstance) (Utilities|String|Append "ThrustUD (" (Utilities|String|ToString(Float) _returnvalue) ")") "(R=0.058824,G=0.615686,B=0.192157,A=1.000000)" 1.0 self "ThrustUD")))
        (else
          (goto _label)))
      ;[0.9844 0.9844 0.9844] Spawn/Create Thrust Exhaust
      (if (> _returnvalue 0.0)
        (Utilities|MacroExhaust (Class|KismetSystemLibrary|MakeLiteralInteger))
        (else
          (Utilities|MacroExhaust (Class|KismetSystemLibrary|MakeLiteralInteger 1))))
      (else
        (CallFunction|CharDie "Fuel")))))

(event Input|EnhancedActionEvents|EnhancedInputActionIA_ThrustX
  (params (ActionValue :type Float%20%28double-precision%29) (ElapsedSeconds :type Float%20%28double-precision%29) (TriggeredSeconds :type Float%20%28double-precision%29) (InputAction :type Input%20Action%20Object%20Reference :default "/Game/Input/IA_ThrustX.IA_ThrustX"))
  (bind _returnvalue (Math|Float|Clamp(Float) ActionValue -1.0))
  (bind _gameinstance (Variables|Default|GetGameInstance))
  (bind _gameinstance_2 (Variables|Default|GetGameInstance))
  (bind _gameinstance_3 (Variables|Default|GetGameInstance))
  (bind _gameinstance_4 (Variables|Default|GetGameInstance))
  (bind _struct_savegame_game (Variables|/Game/Blueprints/CosmosCleaner_GameInstance.CosmosCleaner_GameInstance_C|GetStruct_SaveGame-Game _gameinstance_4))
  (bind _struct_savegame_game_2 (Variables|/Game/Blueprints/CosmosCleaner_GameInstance.CosmosCleaner_GameInstance_C|GetStruct_SaveGame-Game _gameinstance_2))
  (bind _struct_savegame_game_3 (Variables|/Game/Blueprints/CosmosCleaner_GameInstance.CosmosCleaner_GameInstance_C|GetStruct_SaveGame-Game _gameinstance))
  (bind _mousemovement_ (Utilities|Struct|BreakStruct_SaveGame-Game _struct_savegame_game))
  ;[0 0 0] Press RollLeft/RollRight to Roll
  ;[0.9583 0.9583 0.9583] Able to Roll?
  (if (!= _returnvalue 0.0)
    (if (> (Utilities|Struct|BreakStruct_SaveGame-Game (Variables|/Game/Blueprints/CosmosCleaner_GameInstance.CosmosCleaner_GameInstance_C|GetStruct_SaveGame-Game (Variables|Default|GetGameInstance))) 0.0)
      (if (Variables|Boost|GetBoosting?)
        (if (> (- (Variables|/Game/Blueprints/CosmosCleaner_GameInstance.CosmosCleaner_GameInstance_C|GetBoost (Variables|Default|GetGameInstance)) (Variables|Boost|GetBoostRollLossMultiplier)) 0.0)
          (if (not _mousemovement_)
            ;[1 0 0.2812] Roll (Boosted)
            (Class|PrimitiveComponent|AddAngularImpulseinDegrees (Variables|Collision|GetCapsuleComponent) (Math|Vector|MakeVector (* _returnvalue (Variables|MovementRate|GetTurnRate) (Variables|Boost|GetTurnRateBoosted) -1.0) 0.0 0.0) "None" false)
            ;[0 0.4141 1] Set Boost Amnt
            (Variables|/Game/Blueprints/CosmosCleaner_GameInstance.CosmosCleaner_GameInstance_C|SetBoost _gameinstance_3 (- (Variables|/Game/Blueprints/CosmosCleaner_GameInstance.CosmosCleaner_GameInstance_C|GetBoost _gameinstance_3) (Variables|Boost|GetBoostRollLossMultiplier)))
            ;[0.4062 1 0] Set Fuel Amnt
            (Utilities|Struct|SetmembersinStruct_SaveGame-Game _struct_savegame_game_2 (- (Utilities|Struct|BreakStruct_SaveGame-Game _struct_savegame_game_2) (Variables|FuelLoss|GetFuelLossMultiplier)))
            ;[1 0.2462 0.3863] Save Game with Current Values
            (Default|SaveCurrent _gameinstance_2)
            ;[0 1 0.25] DEBUG
            (Default|DebugPrint (Variables|Default|GetGameInstance) (Utilities|String|Append "RollLR-Boosted (" (Utilities|String|ToString(Float) _returnvalue) ")") "(R=0.058824,G=0.615686,B=0.192157,A=1.000000)" 1.0 self "RollLR-Boosted")
            ;[0.9844 0.9844 0.9844] Spawn/Create Roll Exhaust
            (if (> _returnvalue 0.0) :!label _label
              (Utilities|MacroExhaust (Class|KismetSystemLibrary|MakeLiteralInteger 2))
              (else
                (Utilities|MacroExhaust (Class|KismetSystemLibrary|MakeLiteralInteger 3)))))
          (else
            (if (not _mousemovement_) :!label _label_2
              ;[1 0 0.2812] Roll
              (Class|PrimitiveComponent|AddAngularImpulseinDegrees (Variables|Collision|GetCapsuleComponent) (Math|Vector|MakeVector (* _returnvalue (Variables|MovementRate|GetTurnRate) -1.0) 0.0 0.0) "None" false)
              ;[0.4062 1 0] Set Fuel Amnt
              (Utilities|Struct|SetmembersinStruct_SaveGame-Game _struct_savegame_game_3 (- (Utilities|Struct|BreakStruct_SaveGame-Game _struct_savegame_game_3) (Variables|FuelLoss|GetFuelLossMultiplierLesser)))
              ;[1 0.2462 0.3863] Save Game with Current Values
              (Default|SaveCurrent _gameinstance)
              ;[0 1 0.25] DEBUG
              (Default|DebugPrint (Variables|Default|GetGameInstance) (Utilities|String|Append "RollLR (" (Utilities|String|ToString(Float) _returnvalue) ")") "(R=0.058824,G=0.615686,B=0.192157,A=1.000000)" 1.0 self "RollLR")
              (goto _label))))
        (else
          (goto _label_2)))
      (else
        (CallFunction|CharDie "Fuel")))))

(event Input|EnhancedActionEvents|EnhancedInputActionIA_Boost
  (params (ActionValue :type Boolean) (ElapsedSeconds :type Float%20%28double-precision%29) (TriggeredSeconds :type Float%20%28double-precision%29) (InputAction :type Input%20Action%20Object%20Reference :default "/Game/Input/IA_Boost.IA_Boost"))
  ;[0 0 0] Press Boost to Boost
  (:Started
    ;[0.9583 0.9583 0.9583] Boost On
    (Variables|Boost|SetBoosting? true)
    (CallFunction|BoostRegenStart)
    ;[0 1 0.25] DEBUG
    (Default|DebugPrint (Variables|Default|GetGameInstance) "Boost On" "(R=0.058824,G=0.615686,B=0.192157,A=1.000000)" 2.0 self "Boost On"))
  (:Completed
    ;[0.9583 0.9583 0.9583] Boost Off
    (Variables|Boost|SetBoosting? false)
    (CallFunction|BoostRegenStart)
    ;[0 1 0.25] DEBUG
    (Default|DebugPrint (Variables|Default|GetGameInstance) "Boost Off" "(R=0.058824,G=0.615686,B=0.192157,A=1.000000)" 2.0 self "Boost Off")))

(event Custom|CharDie
  (params (Reason :type String))
  (bind _gameinstance (Variables|Default|GetGameInstance))
  (bind _gameinstance_2 (Variables|Default|GetGameInstance))
  (bind _gameinstance_3 (Variables|Default|GetGameInstance))
  (bind _gameinstance_4 (Variables|Default|GetGameInstance))
  (bind _gameinstance_5 (Variables|Default|GetGameInstance))
  (bind _struct_savegame_game (Variables|/Game/Blueprints/CosmosCleaner_GameInstance.CosmosCleaner_GameInstance_C|GetStruct_SaveGame-Game _gameinstance_5))
  (bind _savegamename (Variables|/Game/Blueprints/CosmosCleaner_GameInstance.CosmosCleaner_GameInstance_C|GetSaveGameName _gameinstance_3))
  ;[1 0 0] Kill this Char based on Reason
  (if (Utilities|Array|IsEmpty Reason)
    ;[1 0 0] Destroy Actor
    (Actor|DestroyActor)
    ;[0.9792 0.9792 0.9792] Start New Day
    (Default|LevelNewDay _gameinstance_2)
    ;[0 1 0.25] DEBUG
    (Default|DebugPrint _gameinstance_2 "Character Death" "(R=0.058824,G=0.615686,B=0.192157,A=1.000000)" 2.0 self "CharDie")
    (else
      (switch string Reason
        (:Default
          ;[1 0 0] Destroy Actor
          (Actor|DestroyActor)
          ;[0.9792 0.9792 0.9792] Start New Day
          (Default|LevelNewDay _gameinstance_4)
          ;[0 1 0.25] DEBUG
          (Default|DebugPrint _gameinstance_4 (Utilities|String|Append "Character Death (Reason = " Reason ")") "(R=0.058824,G=0.615686,B=0.192157,A=1.000000)" 2.0 self "CharDie"))
        (:Fuel
          ;[0.9688 0.9688 0.9688] Check for existing savegame
          (bind _returnvalue (SaveGame|DoesSaveGameExist _savegamename))
          (if _returnvalue
            ;[0.9688 0.9688 0.9688] Load existing savegame
            (bind _returnvalue_2 (SaveGame|LoadGamefromSlot _savegamename))
            (bind _assave_game_cosmos_cleaner (Utilities|Casting|CastToSaveGame_CosmosCleaner _returnvalue_2))
            ;[0.9792 0.9792 0.9792] Save Values Changed from Upgrade
            (Utilities|Struct|SetmembersinStruct_SaveGame-Game _struct_savegame_game (Utilities|Struct|BreakStruct_SaveGame-Game (Variables|/Game/Blueprints/SaveGame/SaveGame_CosmosCleaner.SaveGame_CosmosCleaner_C|GetSaveGame-Game_Default _assave_game_cosmos_cleaner)) 0.0 (.FuelMax (Utilities|Struct|BreakStruct_SaveGame-Game _struct_savegame_game)))
            ;[1 0.2462 0.3863] Save Game with Current Values
            (Default|SaveCurrent _gameinstance_5)
            ;[0.9792 0.9792 0.9792] Set Death Reason Text
            (Variables|/Game/Blueprints/CosmosCleaner_GameInstance.CosmosCleaner_GameInstance_C|SetDeath? (Variables|Default|GetGameInstance) "You ran out of fuel! 
Your cargo was lost.")
            ;[0.9792 0.9792 0.9792] Reset Boost to Full
            (Variables|/Game/Blueprints/CosmosCleaner_GameInstance.CosmosCleaner_GameInstance_C|SetBoost (Variables|Default|GetGameInstance) 1e+02)
            ;[0.9792 0.9792 0.9792] Start New Day
            (Default|LevelNewDay _gameinstance)
            ;[0 1 0.25] DEBUG
            (Default|DebugPrint _gameinstance (Utilities|String|Append "Character Death (Reason = " Reason ")") "(R=0.058824,G=0.615686,B=0.192157,A=1.000000)" 2.0 self "CharDie")))))))