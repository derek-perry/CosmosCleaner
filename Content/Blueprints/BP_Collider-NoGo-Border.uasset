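; Border collider that acts as a no-go wall, reacting when the player character hits it.
; On mesh hit it prints a debug message, then plays a collision sound and force feedback if the impulse is non-negligible.
; A gate with a short delay throttles repeated hit feedback.
; A rate-limited "Signal Limit" HUD notification is present but disconnected, so it never runs.
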(event OnComponentHit(Mesh_Area)
  (params (HitComponent :type Primitive%20Component%20Object%20Reference) (OtherActor :type Actor%20Object%20Reference) (OtherComp :type Primitive%20Component%20Object%20Reference) (NormalImpulse :type Vector :default "0, 0, 0") (Hit :type Hit%20Result%20Structure%20%28by%20ref%29))
  (bind (_x _y _z) (Math|Vector|BreakVector NormalImpulse))
  ;[0.9427 0.9427 0.9427] Collider Hit Check - NoGo for Character and Clutter
  (Utilities|Casting|CastToBP_Character OtherActor)
  ;[0 1 0.25] DEBUG
  (bind _ascosmos_cleaner_game_instance (Utilities|Casting|CastToCosmosCleaner_GameInstance (Game|GetGameInstance)))
  (Default|DebugPrint _ascosmos_cleaner_game_instance (Utilities|String|Append "Char Hit" (Variables|Default|GetColliderSide) " Border") "(R=0.058824,G=0.615686,B=0.192157,A=1.000000)" 2.0 self "CharHitBorder")
  ;[0.9583 0.9583 0.9583] Get Impact Velocity
  (Utilities|FlowControl|Sequence
    (:then_0
      (Utilities|FlowControl|Gate false :!label _label
        (:Exit
          (if (not (Math|Boolean|ANDBoolean (Math|Float|NearlyEqual(Float) _x 0.0 1e+02) (Math|Float|NearlyEqual(Float) _y 0.0 1e+02) (Math|Float|NearlyEqual(Float) _z 0.0 1e+02)))
            ;[0.25 0 1] Play Sound : Collide
            (Audio|PlaySound2D "/Game/Audio/SFX/A_Cue_SFX_Collide.A_Cue_SFX_Collide" 1.0 1.0 0.0 0 0 false)
            ;[1 0.1476 0.8785] Play Force Feedback : Collide
            (Game|Feedback|ClientPlayForceFeedback (Game|GetPlayerController 0) "/Game/Input/FFE_Collide.FFE_Collide" "FFE_Collide" false false false)))))
    (:then_1
      (goto _label Close))
    (:then_2
      (Utilities|FlowControl|Delay 0.05)
      (goto _label Open))))

(fn ConstructionScript)