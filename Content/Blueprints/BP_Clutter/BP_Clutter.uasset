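; BP_Clutter is a drifting physics clutter object in Cosmos Cleaner, tracked by the game instance.
; BeginPlay randomizes scale and applies random Y/Z velocity and X-axis spin impulses.
; A dynamic material carries its color, defaulting to white; color updates also check X depth, blacking out off-plane clutter or destroying it when farther out.
; DestroyClutter decrements the game instance's count and calls SpawnClutterMax before removing the actor.
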(event Custom|ChangeColor
  (params (Color :type Linear%20Color%20Structure))
  ;[0.9792 0.9792 0.9792] Check Size for Color Change
  ;[0.9844 0.9844 0.9844] Check is input color is not empty/default
  (if (Class|KismetMathLibrary|LinearColorIsNearEqual :A Color)
    ;[0.9844 0.9844 0.9844] Check is input color is not empty/default
    (if (Class|KismetMathLibrary|LinearColorIsNearEqual :A (Variables|Attributes|GetColor))
      ;[0.9792 0.9792 0.9792] Change Color of Clutter
      (Rendering|Material|SetVectorParameterValue (Variables|Default|GetObstacleMeshMatDyn) "Color" "(R=1.000000,G=1.000000,B=1.000000,A=1.000000)" :!class /Script/Engine.MaterialInstanceDynamic)
      (else
        ;[0.9792 0.9792 0.9792] Change Color of Clutter
        (Rendering|Material|SetVectorParameterValue (Variables|Default|GetObstacleMeshMatDyn) "Color" (Variables|Attributes|GetColor) :!class /Script/Engine.MaterialInstanceDynamic)))
    (else
      ;[0.9792 0.9792 0.9792] Change Color of Clutter
      (Rendering|Material|SetVectorParameterValue (Variables|Default|GetObstacleMeshMatDyn) "Color" Color :!class /Script/Engine.MaterialInstanceDynamic)))
  ;[0.9583 0.9583 0.9583] Within play area/along x-axis?
  (if (not (Math|Float|InRange(Float) (.x (Transformation|GetWorldLocation (Variables|Default|GetMesh_Clutter))) -5e+01 5e+01))
    (if (Math|Float|InRange(Float) (.x (Transformation|GetWorldLocation (Variables|Default|GetMesh_Clutter))) -2.5e+02 2.5e+02)
      (Rendering|Material|SetVectorParameterValue (Variables|Default|GetObstacleMeshMatDyn) "Color" "(R=0.000000,G=0.000000,B=0.000000,A=0.000000)" :!class /Script/Engine.MaterialInstanceDynamic)
      (else
        (Actor|DestroyActor)))))

(event Custom|DestroyClutter
  (bind _gameinstance (Variables|Default|GetGameInstance))
  ;[1 0 0] Destroy This Clutter
  ;[0.9531 0.9531 0.9531] Decrement ClutterAmount
  (Math|Integer|DecrementInt (Variables|/Game/Blueprints/CosmosCleaner_GameInstance.CosmosCleaner_GameInstance_C|GetClutterAmount _gameinstance)
    (:%20%20
      (Default|SpawnClutterMax _gameinstance)
      ;[1 0 0] Destroy Actor
      (Actor|DestroyActor)
      ;[0 1 0.25] DEBUG
      (Default|DebugPrint _gameinstance "Clutter Bordered" "(R=0.058824,G=0.615686,B=0.192157,A=1.000000)" 2.0 self "ClutterBordered"))))

(event EventBeginPlay
  (bind _initialvelocity_roll (Variables|Attributes|GetInitialVelocity_Roll))
  (bind _initialvelocity_y (Variables|Attributes|GetInitialVelocity_Y))
  (bind _initialvelocity_z (Variables|Attributes|GetInitialVelocity_Z))
  (bind _scalevariation (Variables|Attributes|GetScaleVariation))
  (bind (_x _y _z) (Math|Vector|BreakVector _scalevariation))
  (bind _returnvalue (* _initialvelocity_z -1.0))
  (bind _returnvalue_2 (* _initialvelocity_y -1.0))
  (bind _returnvalue_3 (* _initialvelocity_roll -1.0))
  (bind _returnvalue_4 (Math|Random|RandomFloatinRange 1.0 _y))
  (bind _returnvalue_5 (Math|Random|RandomFloatinRange _returnvalue _initialvelocity_z))
  (bind _returnvalue_6 (Math|Random|RandomFloatinRange _returnvalue_3 _initialvelocity_roll))
  (bind _returnvalue_7 (Math|Random|RandomFloatinRange _returnvalue_2 _initialvelocity_y))
  (bind _returnvalue_8 (Math|Random|RandomFloatinRange 1.0 _z))
  (bind _returnvalue_9 (Math|Random|RandomFloatinRange 1.0 _x))
  ;[0 1 0] BeginPlay
  (Utilities|FlowControl|Sequence
    (:then_0
      ;[0.9583 0.9583 0.9583] Get/Set GameInstance Ref
      (bind _ascosmos_cleaner_game_instance (Utilities|Casting|CastToCosmosCleaner_GameInstance (Game|GetGameInstance)))
      (Variables|Default|SetGameInstance _ascosmos_cleaner_game_instance))
    (:then_1
      ;[0.9375 0.9375 0.9375] Get/Set Scale of Clutter (Variation within range)
      (if (Class|KismetMathLibrary|NotEqualExactlyVectorVector _scalevariation "0, 0, 0")
        (Transformation|SetActorScale3D self (Math|Vector|MakeVector _returnvalue_9 _returnvalue_4 _returnvalue_8))
        (Variables|InitialValues|SetInitial_Scale (Math|Vector|MakeVector _returnvalue_9 _returnvalue_4 _returnvalue_8))
        (else
          (Transformation|SetActorScale3D self "1.000000,1.000000,1.000000"))))
    (:then_2
      ;[0.974 0.974 0.974] Set Initial Velocity
      (Physics|AddImpulse (Variables|Default|GetMesh_Clutter) (Math|Vector|MakeVector 0.0 _returnvalue_7 _returnvalue_5) "None" true)
      (Class|PrimitiveComponent|AddAngularImpulseinDegrees (Variables|Default|GetMesh_Clutter) (Math|Vector|MakeVector _returnvalue_6 0.0 0.0) "None" true)
      (Variables|InitialValues|SetInitial_Impulse (Math|Vector|MakeVector 0.0 _returnvalue_7 _returnvalue_5))
      (Variables|InitialValues|SetInitial_ImpulseAngular (Math|Vector|MakeVector _returnvalue_6 0.0 0.0)))
    (:then_3
      ;[0.9844 0.9844 0.9844] Check is input color is not empty/default
      (if (Class|KismetMathLibrary|LinearColorIsNearEqual :A (Variables|Attributes|GetColor))
        ;[0.9792 0.9792 0.9792] Change Color of Clutter
        (Rendering|Material|SetVectorParameterValue (Variables|Default|GetObstacleMeshMatDyn) "Color" "(R=1.000000,G=1.000000,B=1.000000,A=1.000000)" :!class /Script/Engine.MaterialInstanceDynamic)
        (else
          ;[0.9792 0.9792 0.9792] Change Color of Clutter
          (Rendering|Material|SetVectorParameterValue (Variables|Default|GetObstacleMeshMatDyn) "Color" (Variables|Attributes|GetColor) :!class /Script/Engine.MaterialInstanceDynamic)))
      ;[0.9583 0.9583 0.9583] Within play area/along x-axis?
      (if (not (Math|Float|InRange(Float) (.x (Transformation|GetWorldLocation (Variables|Default|GetMesh_Clutter))) -5e+01 5e+01))
        (if (Math|Float|InRange(Float) (.x (Transformation|GetWorldLocation (Variables|Default|GetMesh_Clutter))) -2.5e+02 2.5e+02)
          (Rendering|Material|SetVectorParameterValue (Variables|Default|GetObstacleMeshMatDyn) "Color" "(R=0.000000,G=0.000000,B=0.000000,A=0.000000)" :!class /Script/Engine.MaterialInstanceDynamic)
          (else
            (Actor|DestroyActor)))))
    (:then_4
      ;[0 1 0.25] DEBUG
      (Default|DebugPrint (Variables|Default|GetGameInstance) (Utilities|String|Append "Clutter Created" " (" (Utilities|String|ToString(Integer) (Variables|/Game/Blueprints/CosmosCleaner_GameInstance.CosmosCleaner_GameInstance_C|GetClutterAmount (Variables|Default|GetGameInstance))) "/" (Utilities|String|ToString(Integer) (- (Variables|/Game/Blueprints/CosmosCleaner_GameInstance.CosmosCleaner_GameInstance_C|GetClutterAmountMax (Variables|Default|GetGameInstance)) 1)) ")") "(R=0.058824,G=0.615686,B=0.192157,A=1.000000)" 2.0 self "ClutterCreated"))))

(fn ConstructionScript
  ;[0 1 0] Construct
  ;[0.9792 0.9792 0.9792] Get/Set Dynamic Material
  (Variables|Default|SetObstacleMeshMat (Rendering|Material|GetMaterial (Variables|Default|GetMesh_Clutter) 0))
  (bind _returnvalue (Rendering|Material|CreateDynamicMaterialInstance (Variables|Default|GetMesh_Clutter) 0 (Variables|Default|GetObstacleMeshMat) "MatDyn_Mesh" :!class /Script/Engine.PrimitiveComponent))
  (Variables|Default|SetObstacleMeshMatDyn _returnvalue)
  ;[0.9844 0.9844 0.9844] Check is input color is not empty/default
  (if (Class|KismetMathLibrary|LinearColorIsNearEqual :A (Variables|Attributes|GetColor))
    ;[0.9792 0.9792 0.9792] Change Color of Clutter
    (Rendering|Material|SetVectorParameterValue (Variables|Default|GetObstacleMeshMatDyn) "Color" "(R=1.000000,G=1.000000,B=1.000000,A=1.000000)" :!class /Script/Engine.MaterialInstanceDynamic)
    (else
      ;[0.9792 0.9792 0.9792] Change Color of Clutter
      (Rendering|Material|SetVectorParameterValue (Variables|Default|GetObstacleMeshMatDyn) "Color" (Variables|Attributes|GetColor) :!class /Script/Engine.MaterialInstanceDynamic))))