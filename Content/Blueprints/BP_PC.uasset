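; BP_PC, apparently the player controller, creates the pause and home base widgets and adds them to the viewport.
; The Pause input opens W_Pause only on Map_Game and only if no valid one exists.
; CreateWidgetHomeBase opens W_HomeBase, but its guard checks the pause widget reference rather than the home base one.
; Each creation logs the widget name through GameInstance_All's DebugPrint.
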(event Custom|CreateWidgetHomeBase
  ;[0.9688 0.9688 0.9688] Create Widget HomeBase
  ;[0.974 0.974 0.974] Existing W_HomeBase?
  (Utilities|IsValid (Variables|Default|GetW_Pause)
    (:Is%20Not%20Valid
      ;[0 1 0.25] Create Widget - W_HomeBase
      (bind _returnvalue (UserInterface|CreateWidget "/Game/Widgets/W_HomeBase.W_HomeBase_C"))
      (bind _output_get (Variables|Default|SetW_HomeBase _returnvalue))
      (UserInterface|Viewport|AddtoViewport _output_get 0)
      ;[0 1 0.25] DEBUG
      (bind _asgame_instance_all (Utilities|Casting|CastToGameInstance_All (Game|GetGameInstance)))
      (Default|DebugPrint _asgame_instance_all (Utilities|String|Append "Widget Created (" (Utilities|GetDisplayName _output_get) ")") "(R=0.058824,G=0.615686,B=0.192157,A=1.000000)" 2.0))))

(event Input|ActionEvents|InputActionPause
  (params (Key :type Key%20Structure :default "None"))
  ;[0 0 0] Press Pause Button
  (:Pressed
    ;[0.9688 0.9688 0.9688] Current map is game map?
    (bind _returnvalue (Game|GetCurrentLevelName true))
    (if (Utilities|Enum|Equal(Enum) _returnvalue "Map_Game")
      ;[0.974 0.974 0.974] Existing W_Pause?
      (Utilities|IsValid (Variables|Default|GetW_Pause)
        (:Is%20Not%20Valid
          ;[0 1 0.25] Create Widget - W_Pause
          (bind _returnvalue_2 (UserInterface|CreateWidget "/Game/Widgets/W_Pause.W_Pause_C"))
          (bind _output_get (Variables|Default|SetW_Pause _returnvalue_2))
          (UserInterface|Viewport|AddtoViewport _output_get 0)
          ;[0 1 0.25] DEBUG
          (bind _asgame_instance_all (Utilities|Casting|CastToGameInstance_All (Game|GetGameInstance)))
          (Default|DebugPrint _asgame_instance_all (Utilities|String|Append "Widget Created (" (Utilities|GetDisplayName _output_get) ")") "(R=0.058824,G=0.615686,B=0.192157,A=1.000000)" 2.0))))))

(fn ConstructionScript)