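; Projectile actor that launches itself along the orientation of the player's lander and removes itself after a short lifetime.
; On BeginPlay it caches the BP_Player, then applies a velocity-change impulse to its mesh from the Lander's right vector scaled by BoostMultiplier.
; The impulse uses only the Y and Z components, with no push along X.
; A delay then destroys the actor; the graph has no hit handling.
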(event EventBeginPlay
  (bind _boostmultiplier (Variables|Default|GetBoostMultiplier))
  ;[1 1 1] Save Player
  (bind _asbp_player (Utilities|Casting|CastToBP_Player (Game|GetPlayerCharacter 0)))
  (bind _output_get (Variables|Default|SetPlayer _asbp_player))
  ;[1 1 1] Set Velocity
  (Physics|AddImpulse (Variables|Default|GetProjectileMesh) (Math|Vector|MakeVector 0.0 (* (.y (Math|Vector|GetRightVector (Variables|/Game/Blueprints/BP_Player.BP_Player_C|GetLander _output_get))) _boostmultiplier) (* (.z (Math|Vector|GetRightVector (Variables|/Game/Blueprints/BP_Player.BP_Player_C|GetLander _output_get))) _boostmultiplier)) "None" true)
  ;[1 1 1] Eventually Die
  (Utilities|FlowControl|Delay 5.0)
  (Actor|DestroyActor))

(fn ConstructionScript)