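; Player character that flies with physics thrusters and collects BP_Clutter, destroying it when it begins overlapping a collect area shown while Collect is held.
; Thrust and roll apply capsule impulses that drain GameInstance_All's Fuel, with Boost strengthening them while its charge lasts.
; Boost press and release each start a recursive Delay loop that refills charge.
; Scroll zooms the spring arm, saving its length to the game instance.
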(event EventBeginPlay
  ;[0 1 0] BeginPlay
  ;[0.9635 0.9635 0.9635] Reset Velocity
  (Variables|/Script/Engine.MovementComponent|SetVelocity (Variables|Character|GetCharacterMovement) "0, 0, 0")
  ;[0.9635 0.9635 0.9635] Save Game Instance
  (bind _asgame_instance_all (Utilities|Casting|CastToGameInstance_All (Game|GetGameInstance))
    (:then
      (bind _output_get (Variables|Default|SetGameInstance_All _asgame_instance_all))
      ;[0.9531 0.9531 0.9531] Set Camera's Arm Length based on Scroll Input
      (Variables|/Script/Engine.SpringArmComponent|SetTargetArmLength (Variables|Default|GetSpringArm_Camera) (Variables|/Game/Blueprints/GameInstance_All.GameInstance_All_C|GetCameraScrollLength _output_get)))
    (:CastFailed
      _))
  ;[0 1 0.25] DEBUG
  (Default|DebugPrint _output_get "Player Created" "(R=0.058824,G=0.615686,B=0.192157,A=1.000000)" 2.0 self "None"))

(fn ConstructionScript)

(event OnComponentBeginOverlap(Mesh_CollectArea)
  (params (OverlappedComponent :type Primitive%20Component%20Object%20Reference) (OtherActor :type Actor%20Object%20Reference) (OtherComp :type Primitive%20Component%20Object%20Reference) (OtherBodyIndex :type Integer) (bFromSweep :type Boolean) (SweepResult :type Hit%20Result%20Structure%20%28by%20ref%29))
  ;[0.9792 0.9792 0.9792] Collider Check - Collect Area
  (bind _asbp_clutter (Utilities|Casting|CastToBP_Clutter OtherActor))
  (Default|DestroyClutter _asbp_clutter)
  ;[0 1 0.25] DEBUG
  (Default|DebugPrint (Variables|Default|GetGameInstance_All) "Clutter Collected" "(R=0.058824,G=0.615686,B=0.192157,A=1.000000)" 2.0 self "None"))

(event OnComponentEndOverlap(Mesh_CollectArea)
  (params (OverlappedComponent :type Primitive%20Component%20Object%20Reference) (OtherActor :type Actor%20Object%20Reference) (OtherComp :type Primitive%20Component%20Object%20Reference) (OtherBodyIndex :type Integer))
  ;[0.9792 0.9792 0.9792] Collider Check - Collect Area
  (Utilities|Casting|CastToBP_Clutter OtherActor)
  ;[0 1 0.25] DEBUG
  (Default|DebugPrint (Variables|Default|GetGameInstance_All) "Clutter Stopped Overlapping Collect Area" "(R=0.058824,G=0.615686,B=0.192157,A=1.000000)" 2.0 self "None"))

(event Input|ActionEvents|InputActionCollect
  (params (Key :type Key%20Structure :default "None"))
  ;[0 0 0] Collect
  (:Pressed
    ;[0.974 0.974 0.974] Set isCollecting? and Show/Hide CollectArea
    (Development|SetHiddeninGame (Variables|Default|GetMesh_CollectArea) false true)
    (Variables|Default|SetisCollecting? true)
    ;[0 1 0.25] DEBUG
    (Default|DebugPrint (Variables|Default|GetGameInstance_All) "Collection Started" "(R=0.058824,G=0.615686,B=0.192157,A=1.000000)" 2.0 self "None"))
  (:Released
    ;[0.974 0.974 0.974] Set isCollecting? and Show/Hide CollectArea
    (Development|SetHiddeninGame (Variables|Default|GetMesh_CollectArea) true true)
    (Variables|Default|SetisCollecting? false)
    ;[0 1 0.25] DEBUG
    (Default|DebugPrint (Variables|Default|GetGameInstance_All) "Collection Stopped" "(R=0.058824,G=0.615686,B=0.192157,A=1.000000)" 2.0 self "None")))

(event Custom|BoostRegenStart
  (bind _gameinstance_all (Variables|Default|GetGameInstance_All))
  ;[0.9688 0.9688 0.9688] Regenerate Boost Over Time
  (if (< (Variables|/Game/Blueprints/GameInstance_All.GameInstance_All_C|GetBoost _gameinstance_all) 99.475)
    (Variables|/Game/Blueprints/GameInstance_All.GameInstance_All_C|SetBoost _gameinstance_all (+ (Variables|/Game/Blueprints/GameInstance_All.GameInstance_All_C|GetBoost _gameinstance_all) 0.525))
    (Utilities|FlowControl|Delay 0.01)
    (CallFunction|BoostRegenStart)
    (elif (< (Variables|/Game/Blueprints/GameInstance_All.GameInstance_All_C|GetBoost _gameinstance_all) 1e+02)
      (Variables|/Game/Blueprints/GameInstance_All.GameInstance_All_C|SetBoost _gameinstance_all 1e+02))))

(event Input|ActionEvents|InputActionBoost
  (params (Key :type Key%20Structure :default "None"))
  ;[0 0 0] Press Boost to Boost
  (:Pressed
    ;[0.9583 0.9583 0.9583] Boost On
    (Variables|Movement|SetBoosting? true)
    (CallFunction|BoostRegenStart)
    ;[0 1 0.25] DEBUG
    (Default|DebugPrint (Variables|Default|GetGameInstance_All) "Boost On" "(R=0.058824,G=0.615686,B=0.192157,A=1.000000)" 2.0 self "None"))
  (:Released
    ;[0.9583 0.9583 0.9583] Boost Off
    (Variables|Movement|SetBoosting? false)
    (CallFunction|BoostRegenStart)
    ;[0 1 0.25] DEBUG
    (Default|DebugPrint (Variables|Default|GetGameInstance_All) "Boost Off" "(R=0.058824,G=0.615686,B=0.192157,A=1.000000)" 2.0 self "None")))

(event Input|AxisEvents|InputAxisLeft/Right
  (params (AxisValue :type Float%20%28single-precision%29))
  (bind _returnvalue (Math|Float|Clamp(Float) AxisValue -1.0))
  (bind _gameinstance_all (Variables|Default|GetGameInstance_All))
  (bind _gameinstance_all_2 (Variables|Default|GetGameInstance_All))
  (bind _gameinstance_all_3 (Variables|Default|GetGameInstance_All))
  ;[0 0 0] Press RollLeft/RollRight to Roll
  ;[0.9583 0.9583 0.9583] Able to Roll?
  (if (!= _returnvalue 0.0)
    (if (> (Variables|/Game/Blueprints/GameInstance_All.GameInstance_All_C|GetFuel (Variables|Default|GetGameInstance_All)) 0.0)
      (if (Variables|Movement|GetBoosting?)
        (if (> (- (Variables|/Game/Blueprints/GameInstance_All.GameInstance_All_C|GetBoost (Variables|Default|GetGameInstance_All)) (Variables|Movement|GetBoostRollLossMultiplier)) 0.0)
          ;[1 0 0.2812] Roll (Boosted)
          (Class|PrimitiveComponent|AddAngularImpulseinDegrees (Variables|Collision|GetCapsuleComponent) (Math|Vector|MakeVector (* _returnvalue (Variables|Movement|GetTurnRate) (Variables|Movement|GetTurnRateBoosted) -1.0) 0.0 0.0) "None" false)
          ;[0 0.4141 1] Set Boost Amnt
          (Variables|/Game/Blueprints/GameInstance_All.GameInstance_All_C|SetBoost _gameinstance_all_3 (- (Variables|/Game/Blueprints/GameInstance_All.GameInstance_All_C|GetBoost _gameinstance_all_3) (Variables|Movement|GetBoostRollLossMultiplier)))
          ;[0.4062 1 0] Set Fuel Amnt
          (Variables|/Game/Blueprints/GameInstance_All.GameInstance_All_C|SetFuel _gameinstance_all_2 (- (Variables|/Game/Blueprints/GameInstance_All.GameInstance_All_C|GetFuel _gameinstance_all_2) (Variables|Fuel|GetFuelLossMultiplierLesser)))
          ;[0 1 0.25] DEBUG
          (Default|DebugPrint (Variables|Default|GetGameInstance_All) (Utilities|String|Append "RollLR-Boosted (" (Utilities|String|ToString(Float) _returnvalue) ")") "(R=0.058824,G=0.615686,B=0.192157,A=1.000000)" 1.0 self "None")
          (else
            ;[1 0 0.2812] Roll
            (Class|PrimitiveComponent|AddAngularImpulseinDegrees (Variables|Collision|GetCapsuleComponent) (Math|Vector|MakeVector (* _returnvalue (Variables|Movement|GetTurnRate) -1.0) 0.0 0.0) "None" false :!label _label)
            ;[0.4062 1 0] Set Fuel Amnt
            (Variables|/Game/Blueprints/GameInstance_All.GameInstance_All_C|SetFuel _gameinstance_all (- (Variables|/Game/Blueprints/GameInstance_All.GameInstance_All_C|GetFuel _gameinstance_all) (Variables|Fuel|GetFuelLossMultiplierLesser)))
            ;[0 1 0.25] DEBUG
            (Default|DebugPrint (Variables|Default|GetGameInstance_All) (Utilities|String|Append "RollLR (" (Utilities|String|ToString(Float) _returnvalue) ")") "(R=0.058824,G=0.615686,B=0.192157,A=1.000000)" 1.0 self "None")))
        (else
          (goto _label))))))

(event Input|AxisEvents|InputAxisUp/Down
  (params (AxisValue :type Float%20%28single-precision%29))
  (bind _returnvalue (Math|Float|Clamp(Float) AxisValue -0.75))
  (bind _self self)
  (bind _self_2 self)
  (bind _gameinstance_all (Variables|Default|GetGameInstance_All))
  (bind _gameinstance_all_2 (Variables|Default|GetGameInstance_All))
  (bind _thrustermultiplier (Variables|Movement|GetThrusterMultiplier))
  (bind _thrustermultiplier_2 (Variables|Movement|GetThrusterMultiplier))
  (bind _boostthrustmultiplier (Variables|Movement|GetBoostThrustMultiplier))
  (bind _gameinstance_all_3 (Variables|Default|GetGameInstance_All))
  (bind _fuellossmultiplier (Variables|Fuel|GetFuelLossMultiplier))
  (bind _returnvalue_2 (Transformation|GetActorUpVector _self_2))
  (bind _returnvalue_3 (Transformation|GetActorUpVector _self))
  (bind _returnvalue_4 (* _returnvalue _thrustermultiplier))
  (bind _returnvalue_5 (* _returnvalue _thrustermultiplier_2 _boostthrustmultiplier))
  ;[0 0 0] Press Up/Down to Thrust
  ;[0.9531 0.9531 0.9531] Able to Thrust?
  (if (!= _returnvalue 0.0)
    (if (> (Variables|/Game/Blueprints/GameInstance_All.GameInstance_All_C|GetFuel (Variables|Default|GetGameInstance_All)) 0.0)
      (if (Variables|Movement|GetBoosting?)
        (if (> (- (Variables|/Game/Blueprints/GameInstance_All.GameInstance_All_C|GetBoost (Variables|Default|GetGameInstance_All)) (Variables|Movement|GetBoostUDLossMultiplier)) 0.0)
          ;[1 0 0.2812] ThrustUD (Boosted)
          (Physics|AddImpulse (Variables|Collision|GetCapsuleComponent) (Math|Vector|MakeVector (* (.x _returnvalue_3) _returnvalue_5) (* (.y _returnvalue_3) _returnvalue_5) (* (.z _returnvalue_3) _returnvalue_5)) "None" false)
          ;[0 0.4141 1] Set Boost Amnt
          (Variables|/Game/Blueprints/GameInstance_All.GameInstance_All_C|SetBoost _gameinstance_all_3 (- (Variables|/Game/Blueprints/GameInstance_All.GameInstance_All_C|GetBoost _gameinstance_all_3) (Variables|Movement|GetBoostUDLossMultiplier)))
          ;[0.4062 1 0] Set Fuel Amnt
          (Variables|/Game/Blueprints/GameInstance_All.GameInstance_All_C|SetFuel _gameinstance_all_2 (- (Variables|/Game/Blueprints/GameInstance_All.GameInstance_All_C|GetFuel _gameinstance_all_2) (+ _fuellossmultiplier (* _fuellossmultiplier 0.36666))))
          ;[0 1 0.25] DEBUG
          (Default|DebugPrint (Variables|Default|GetGameInstance_All) (Utilities|String|Append "ThrustUD-Boosted (" (Utilities|String|ToString(Float) _returnvalue) ")") "(R=0.058824,G=0.615686,B=0.192157,A=1.000000)" 1.0 self "None")
          (else
            ;[1 0 0.2812] ThrustUD
            (Physics|AddImpulse (Variables|Collision|GetCapsuleComponent) (Math|Vector|MakeVector (* (.x _returnvalue_2) _returnvalue_4) (* (.y _returnvalue_2) _returnvalue_4) (* (.z _returnvalue_2) _returnvalue_4)) "None" false :!label _label)
            ;[0.4062 1 0] Set Fuel Amnt
            (Variables|/Game/Blueprints/GameInstance_All.GameInstance_All_C|SetFuel _gameinstance_all (- (Variables|/Game/Blueprints/GameInstance_All.GameInstance_All_C|GetFuel _gameinstance_all) (Variables|Fuel|GetFuelLossMultiplier)))
            ;[0 1 0.25] DEBUG
            (Default|DebugPrint (Variables|Default|GetGameInstance_All) (Utilities|String|Append "ThrustUD (" (Utilities|String|ToString(Float) _returnvalue) ")") "(R=0.058824,G=0.615686,B=0.192157,A=1.000000)" 1.0 self "None")))
        (else
          (goto _label))))))

(event Input|ActionEvents|InputActionScrollReset
  (params (Key :type Key%20Structure :default "None"))
  ;[0 0 0] ScrollReset
  (:Pressed
    ;[0.9531 0.9531 0.9531] Reset Camera's Arm Length to Default
    (Variables|/Script/Engine.SpringArmComponent|SetTargetArmLength (Variables|Default|GetSpringArm_Camera) 1.5e+03)
    (Variables|/Game/Blueprints/GameInstance_All.GameInstance_All_C|SetCameraScrollLength (Variables|Default|GetGameInstance_All) 1.5e+03)
    ;[0 1 0.25] DEBUG
    (Default|DebugPrint (Variables|Default|GetGameInstance_All) "Camera Scroll Reset" "(R=0.058824,G=0.615686,B=0.192157,A=1.000000)" 2.0 self "None")))

(event Input|AxisEvents|InputAxisScroll
  (params (AxisValue :type Float%20%28single-precision%29))
  (bind _gameinstance_all (Variables|Default|GetGameInstance_All))
  (bind _springarm_camera (Variables|Default|GetSpringArm_Camera))
  ;[0 0 0] Scroll
  ;[0.9531 0.9531 0.9531] Set Camera's Arm Length based on Scroll Input
  (if (!= AxisValue 0.0)
    (if (<= (Variables|/Script/Engine.SpringArmComponent|GetTargetArmLength _springarm_camera) (Variables|Camera|GetCameraScrollMax))
      (if (>= (Variables|/Script/Engine.SpringArmComponent|GetTargetArmLength _springarm_camera) (Variables|Camera|GetCameraScrollMin))
        (Variables|/Script/Engine.SpringArmComponent|SetTargetArmLength _springarm_camera (+ (Variables|/Script/Engine.SpringArmComponent|GetTargetArmLength _springarm_camera) (* AxisValue (Variables|Camera|GetCameraScrollMultiplier) -1.0)))
        (else
          (Variables|/Script/Engine.SpringArmComponent|SetTargetArmLength _springarm_camera (Variables|Camera|GetCameraScrollMin))))
      (else
        (Variables|/Script/Engine.SpringArmComponent|SetTargetArmLength _springarm_camera (Variables|Camera|GetCameraScrollMax))))
    (Variables|/Game/Blueprints/GameInstance_All.GameInstance_All_C|SetCameraScrollLength _gameinstance_all (Variables|/Script/Engine.SpringArmComponent|GetTargetArmLength (Variables|Default|GetSpringArm_Camera)))
    ;[0 1 0.25] DEBUG
    (Default|DebugPrint _gameinstance_all (Utilities|String|Append "Camera Scroll Changed (" (Utilities|String|ToString(Float) (Variables|/Script/Engine.SpringArmComponent|GetTargetArmLength (Variables|Default|GetSpringArm_Camera))) ")") "(R=0.058824,G=0.615686,B=0.192157,A=1.000000)" 2.0 self "CameraScroll")))