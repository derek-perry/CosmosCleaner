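; BP_SpawnerArea is a volume that scatters a set number of clutter objects of one type when play begins.
; It picks random points within the AreaSpawn bounds and asks the Cosmos Cleaner GameInstance to spawn the configured amount at each, with random rotation.
; The loop recurses through the SpawnClutter event until the remaining count reaches zero, and halts early if a point lands on the world origin.
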(event Custom|SpawnClutter
  (bind _returnvalue (Math|Random|RandomFloatinRange -3.6e+02 3.6e+02))
  (bind _area_spawn (Variables|Default|GetArea_Spawn))
  (bind (_origin _boxextent) (Collision|GetComponentBounds _area_spawn))
  ;[0 1 0.7188] Spawn correct amount of Clutters
  (if (Math|Boolean|ANDBoolean (> (Variables|SpawnOptions|GetSpawnCount) 0) (> (Variables|SpawnOptions|GetSpawnCountRemaining) 0) (not (Utilities|Enum|Equal(Enum) (Variables|SpawnOptions|GetSpawnType) "")))
    (Variables|SpawnOptions|SetSpawnTransformLocation (Math|Random|RandomPointinBoundingBox _origin _boxextent))
    (if (not (Class|KismetMathLibrary|EqualExactlyVectorVector (Variables|SpawnOptions|GetSpawnTransformLocation) "0, 0, 0"))
      (Default|SpawnClutterSingle (Variables|Default|GetGameInstance) (Variables|SpawnOptions|GetSpawnType) (Math|Transform|MakeTransform (Variables|SpawnOptions|GetSpawnTransformLocation) (Math|Rotator|MakeRotator _returnvalue _returnvalue _returnvalue) "1.000000,1.000000,1.000000") (Variables|SpawnOptions|GetSpawnAmount))
      (Math|Integer|DecrementInt (Variables|SpawnOptions|GetSpawnCountRemaining)
        (:%20%20
          (CallFunction|SpawnClutter))))))

(event EventBeginPlay
  (bind _returnvalue (Math|Random|RandomFloatinRange -3.6e+02 3.6e+02))
  (bind _area_spawn (Variables|Default|GetArea_Spawn))
  (bind (_origin _boxextent) (Collision|GetComponentBounds _area_spawn))
  ;[0 1 0] Begin Play
  ;[0.9635 0.9635 0.9635] Get/Set GameInstance Ref
  (bind _ascosmos_cleaner_game_instance (Utilities|Casting|CastToCosmosCleaner_GameInstance (Game|GetGameInstance)))
  (Variables|Default|SetGameInstance _ascosmos_cleaner_game_instance)
  ;[0 1 0.7188] Spawn correct amount of Clutters
  (Variables|SpawnOptions|SetSpawnCountRemaining (Variables|SpawnOptions|GetSpawnCount))
  (if (Math|Boolean|ANDBoolean (> (Variables|SpawnOptions|GetSpawnCount) 0) (> (Variables|SpawnOptions|GetSpawnCountRemaining) 0) (not (Utilities|Enum|Equal(Enum) (Variables|SpawnOptions|GetSpawnType) "")))
    (Variables|SpawnOptions|SetSpawnTransformLocation (Math|Random|RandomPointinBoundingBox _origin _boxextent))
    (if (not (Class|KismetMathLibrary|EqualExactlyVectorVector (Variables|SpawnOptions|GetSpawnTransformLocation) "0, 0, 0"))
      (Default|SpawnClutterSingle (Variables|Default|GetGameInstance) (Variables|SpawnOptions|GetSpawnType) (Math|Transform|MakeTransform (Variables|SpawnOptions|GetSpawnTransformLocation) (Math|Rotator|MakeRotator _returnvalue _returnvalue _returnvalue) "1.000000,1.000000,1.000000") (Variables|SpawnOptions|GetSpawnAmount))
      (Math|Integer|DecrementInt (Variables|SpawnOptions|GetSpawnCountRemaining)
        (:%20%20
          (CallFunction|SpawnClutter))))))

(fn ConstructionScript)