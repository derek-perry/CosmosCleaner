(event Custom|StartUp
  (params (MenuOrGame? :type Boolean))
  (bind _savegamename (Variables|SaveGame|GetSaveGameName))
  ;[0 1 0] Start Up Checks
  ;[1 0.2462 0.3863] Check for Save Game (Either Load Existing or Create New)
  (bind _returnvalue (SaveGame|DoesSaveGameExist _savegamename))
  (if _returnvalue
    (bind _returnvalue_2 (SaveGame|LoadGamefromSlot _savegamename))
    (bind _assave_game_all (Utilities|Casting|CastToSaveGame_All _returnvalue_2)
      (:then
        ;[0.9531 0.9531 0.9531] Get/Set SaveGame Structure
        (Variables|SaveGame|SetStruct_SaveGame (Variables|/Game/Blueprints/SaveGame_All.SaveGame_All_C|GetStruct_SaveGame _assave_game_all))
        ;[0.9531 0.9531 0.9531] Get/Set SaveGame Data
        (CallFunction|AudioVolumeGetSet)
        (CallFunction|GameUserSettingsGetSet)
        ;[0.974 0.974 0.974] Menu=True  or  Game=False
        (if MenuOrGame?
          ;[0.9792 0.9792 0.9792] False=Menu Start, True=Going to Menus from Game
          (if (Variables|In-Game|GetComingFromGame?)
            ;[0 1 0.25] Create Widget - Existing Player Coming from In-Game: Main Menu
            (bind _returnvalue_3 (UserInterface|CreateWidget "/Game/Widgets/W_Menu-Main.W_Menu-Main_C"))
            (UserInterface|Viewport|AddtoViewport _returnvalue_3 0)
            (else
              ;[0 1 0.25] Create Widget - Existing Player from Menu Start: Splash, then Main Menu
              (bind _returnvalue_4 (UserInterface|CreateWidget "/Game/Widgets/W_Splash.W_Splash_C"))
              (UserInterface|Viewport|AddtoViewport _returnvalue_4 0)
              (Variables|/Game/Widgets/W_Splash.W_Splash_C|SetNextWidget _returnvalue_4 "/Game/Widgets/W_Menu-Main.W_Menu-Main_C")))
          (else
            ;[1 0.8203 0] Set Input Mode to Game
            (CallFunction|InputModeGame)
            ;[0 1 0.7188] Spawn/Save Ref BP_CET (Player)
            (CallFunction|SaveRefCet)
            ;[0 1 0.7188] Spawn/Save Ref BP_HomeBase
            (CallFunction|SpawnHomeBase)
            ;[0 1 0.7188] Spawn Max Amount of Clutter
            (CallFunction|SpawnClutterMax)
            ;[0 1 0.25] Create Widget - HUD
            (CallFunction|WidgetCreateHUD))))
      (:CastFailed
        (bind _returnvalue_5 (SaveGame|CreateSaveGameObject (Variables|SaveGame|GetSaveGameClass) :!label _label))
        (SaveGame|SaveGametoSlot _returnvalue_5 _savegamename)
        (bind _assave_game_all_2 (Utilities|Casting|CastToSaveGame_All _returnvalue_5)
          (:then
            ;[0.9531 0.9531 0.9531] Get/Set SaveGame Structure
            (Variables|SaveGame|SetStruct_SaveGame (Variables|/Game/Blueprints/SaveGame_All.SaveGame_All_C|GetStruct_SaveGame _assave_game_all_2))
            ;[0.9531 0.9531 0.9531] Get/Set SaveGame Data
            (CallFunction|AudioVolumeGetSet)
            (CallFunction|GameUserSettingsGetSet)
            ;[0.974 0.974 0.974] Menu=True  or  Game=False
            (if MenuOrGame?
              ;[0 1 0.25] Create Widget - First Play: Splash, then Menu-Settings, then Menu-Color, then Main Menu
              (bind _returnvalue_6 (UserInterface|CreateWidget "/Game/Widgets/W_Splash.W_Splash_C"))
              (UserInterface|Viewport|AddtoViewport _returnvalue_6 0)
              (Variables|/Game/Widgets/W_Splash.W_Splash_C|SetNextWidget _returnvalue_6 "/Game/Widgets/W_Menu-Settings.W_Menu-Settings_C")
              (else
                ;[1 0 0.7031] PAUSE
                (Game|SetGamePaused true)
                ;[0 1 0.25] Create Widget - First Play: Menu-Settings, then Pause
                (bind _returnvalue_7 (UserInterface|CreateWidget "/Game/Widgets/W_Menu-Settings.W_Menu-Settings_C"))
                (UserInterface|Viewport|AddtoViewport _returnvalue_7 0)
                (Variables|/Game/Widgets/W_Menu-Settings.W_Menu-Settings_C|SetNextWidget _returnvalue_7 "/Game/Widgets/W_Pause.W_Pause_C"))))
          (:CastFailed
            (goto _label)))))
    (else
      (goto _label))))

(event Custom|GameUserSettingsGetSet
  (bind _struct_savegame (Variables|SaveGame|GetStruct_SaveGame))
  (bind (_videoframeratelimit _vsync_ _debug_) (Utilities|Struct|BreakStruct_SaveGame _struct_savegame))
  ;[1 0.8203 0] Get/Set User Settings (Save/Apply FrameRateLimit and VSync)
  (bind _returnvalue (Settings|GetGameUserSettings))
  (Class|GameUserSettings|SetFrameRateLimit _returnvalue _videoframeratelimit)
  (Class|GameUserSettings|SetVSyncEnabled _returnvalue _vsync_)
  (Class|GameUserSettings|ApplySettings _returnvalue true)
  (Class|GameUserSettings|SaveSettings _returnvalue)
  ;[0 1 0.25] DEBUG
  (if _debug_
    (Development|ExecuteConsoleCommand "EnableAllScreenMessages" 0)
    (else
      (Development|ExecuteConsoleCommand "DisableAllScreenMessages" 0))))

(event Custom|WidgetCreateHUD
  ;[0 1 0.25] Create Widget - HUD
  (bind _returnvalue (UserInterface|CreateWidget "/Game/Widgets/W_HUD.W_HUD_C"))
  (bind _output_get (Variables|Widgets|SetW_HUD _returnvalue))
  (UserInterface|Viewport|AddtoViewport _output_get 0)
  ;[0 1 0.25] DEBUG
  (CallFunction|DebugPrint (Utilities|String|Append "HUD Widget Created (" (Utilities|GetDisplayName _output_get) ")") "(R=0.058824,G=0.615686,B=0.192157,A=1.000000)" 2.0))

(event Custom|MusicStop
  (bind _sound_music_component (Variables|Audio|GetSound_Music-Component))
  ;[0.25 0 1] Stop Music
  (Utilities|IsValid _sound_music_component
    (:Is%20Valid
      (Audio|Components|Audio|Stop _sound_music_component)
      (Components|DestroyComponent _sound_music_component)
      ;[0 1 0.25] DEBUG
      (CallFunction|DebugPrint (Utilities|String|Append "Music Stopped (" (Utilities|GetDisplayName _sound_music_component) ")") "(R=0.058824,G=0.615686,B=0.192157,A=1.000000)" 2.0))))

(event Custom|AudioVolumeGetSet
  (bind _struct_savegame (Variables|SaveGame|GetStruct_SaveGame))
  (bind (_audiomuted _audiosfx _audiomusic _audioambient) (Utilities|Struct|BreakStruct_SaveGame _struct_savegame))
  ;[0.25 0 1] Get/Set Audio Volumes
  (if _audiomuted
    (Class|GameplayStatics|SetBaseSoundMix "/Game/Audio/A_Mix_Mute.A_Mix_Mute")
    (Audio|SetSoundMixClassOverride "/Game/Audio/A_Mix_Mute.A_Mix_Mute" "/Game/Audio/A_SoundClass_SFX.A_SoundClass_SFX" 1e-06 1.0 0.0 true)
    (Audio|SetSoundMixClassOverride "/Game/Audio/A_Mix_Mute.A_Mix_Mute" "/Game/Audio/A_SoundClass_Music.A_SoundClass_Music" 1e-06 1.0 0.0 true)
    (Audio|SetSoundMixClassOverride "/Game/Audio/A_Mix_Mute.A_Mix_Mute" "/Game/Audio/A_SoundClass_Ambient.A_SoundClass_Ambient" 1e-06 1.0 0.0 true)
    (else
      (Class|GameplayStatics|SetBaseSoundMix "/Game/Audio/A_Mix_Default.A_Mix_Default")
      (Audio|SetSoundMixClassOverride "/Game/Audio/A_Mix_Default.A_Mix_Default" "/Game/Audio/A_SoundClass_SFX.A_SoundClass_SFX" _audiosfx 1.0 0.0 true)
      (Audio|SetSoundMixClassOverride "/Game/Audio/A_Mix_Default.A_Mix_Default" "/Game/Audio/A_SoundClass_Music.A_SoundClass_Music" _audiomusic 1.0 0.0 true)
      (Audio|SetSoundMixClassOverride "/Game/Audio/A_Mix_Default.A_Mix_Default" "/Game/Audio/A_SoundClass_Ambient.A_SoundClass_Ambient" _audioambient 1.0 0.0 true))))

(event Custom|MusicPlay
  (params (SoundBase :type Sound%20Base%20Object%20Reference))
  ;[0.25 0 1] Play Music
  (Utilities|IsValid SoundBase
    (:Is%20Valid
      (Utilities|IsValid (Variables|Audio|GetSound_Music)
        (:Is%20Valid
          (if (not (== SoundBase (Variables|Audio|GetSound_Music)))
            (Utilities|FlowControl|Sequence :!label _label
              (:then_0
                (CallFunction|MusicStop))
              (:then_1
                (bind _output_get (Variables|Audio|SetSound_Music SoundBase))
                (bind _returnvalue (Audio|SpawnSound2D _output_get 1.0 1.0 0.0 0))
                (Variables|Audio|SetSound_Music-Component _returnvalue)))))
        (:Is%20Not%20Valid
          (goto _label))))))

(event Custom|SaveCurrentValues
  (bind _savegamename (Variables|SaveGame|GetSaveGameName))
  ;[1 0.2462 0.3863] Save Game with Current Values
  ;[1 0.2462 0.3863] Save Game with Current Values
  (bind _returnvalue (SaveGame|DoesSaveGameExist _savegamename))
  (if _returnvalue
    (bind _returnvalue_2 (SaveGame|LoadGamefromSlot _savegamename))
    (bind _assave_game_all (Utilities|Casting|CastToSaveGame_All _returnvalue_2)
      (:then
        (Variables|/Game/Blueprints/SaveGame_All.SaveGame_All_C|SetStruct_SaveGame _assave_game_all (Variables|SaveGame|GetStruct_SaveGame))
        (SaveGame|SaveGametoSlot _assave_game_all _savegamename))
      (:CastFailed
        (bind _returnvalue_3 (SaveGame|CreateSaveGameObject (Variables|SaveGame|GetSaveGameClass) :!label _label))
        (bind _assave_game_all_2 (Utilities|Casting|CastToSaveGame_All _returnvalue_3))
        (Variables|/Game/Blueprints/SaveGame_All.SaveGame_All_C|SetStruct_SaveGame _assave_game_all_2 (Variables|SaveGame|GetStruct_SaveGame))
        (SaveGame|SaveGametoSlot _assave_game_all_2 _savegamename)))
    (else
      (goto _label))))

(event Custom|InputModeGame
  (bind _returnvalue (Game|GetPlayerController 0))
  ;[1 0.8203 0] Set Input Mode to Game
  (Input|SetInputModeGameOnly _returnvalue false)
  (Variables|/Script/Engine.PlayerController|SetbEnableClickEvents _returnvalue false)
  (Variables|/Script/Engine.PlayerController|SetbEnableMouseOverEvents _returnvalue false)
  (Variables|/Script/Engine.PlayerController|SetbEnableTouchEvents _returnvalue false)
  (Variables|/Script/Engine.PlayerController|SetbEnableTouchOverEvents _returnvalue false)
  (Variables|/Script/Engine.PlayerController|SetbShowMouseCursor _returnvalue false)
  ;[0 1 0.25] DEBUG
  (CallFunction|DebugPrint (Utilities|String|Append "Input Mode Changed to Game using PC(" (Utilities|GetDisplayName _returnvalue) ")") "(R=0.058824,G=0.615686,B=0.192157,A=1.000000)" 2.0))

(event Custom|SpawnClutterMax
  ;[0 1 0.7188] Spawn Max Amount of Clutter
  (if (< (Variables|In-Game|GetClutterAmount) (Variables|In-Game|GetClutterAmountMax)) :!label _label
    (CallFunction|SpawnClutter)
    (goto _label)))

(event Custom|SaveRefCet
  ;[0 1 0.7188] Save/Spawn Ref BP_CET (Player)
  (bind _asbp_cet (Utilities|Casting|CastToBP_CET (Game|GetPlayerCharacter 0))
    (:then
      (bind _output_get (Variables|BPRefs|SetBP_CET-ref _asbp_cet))
      (Transformation|SetActorLocationAndRotation _output_get "0, 0,50.000000" "0, 0, 0" false true)
      ;[0 1 0.25] DEBUG
      (CallFunction|DebugPrint (Utilities|String|Append "BP Ref Saved (" (Utilities|GetDisplayName _output_get) ")") "(R=0.058824,G=0.615686,B=0.192157,A=1.000000)" 2.0))
    (:CastFailed
      (bind _returnvalue (Game|SpawnActorfromClass "/Game/Blueprints/BP_CET.BP_CET_C" (Math|Transform|MakeTransform "0, 0,50.000000" "0, 0, 0" "1.000000,1.000000,1.000000") "Undefined" "MultiplyWithRoot" 0 0))
      (bind _output_get_2 (Variables|BPRefs|SetBP_CET-ref _returnvalue))
      ;[0 1 0.25] DEBUG
      (CallFunction|DebugPrint (Utilities|String|Append "BP Spawned/Ref Saved (" (Utilities|GetDisplayName _output_get_2) ")") "(R=0.058824,G=0.615686,B=0.192157,A=1.000000)" 2.0))))

(event Custom|SpawnHomeBase
  ;[0 1 0.7188] Spawn/Save Ref BP_HomeBase
  (bind _returnvalue (Game|SpawnActorfromClass "/Game/Blueprints/BP_HomeBase.BP_HomeBase_C" (Math|Transform|MakeTransform "0.000000,0.000000,124.000000" "0, 0, 0" "1.000000,1.000000,1.000000") "Undefined" "OverrideRootScale" 0 0))
  (bind _output_get (Variables|BPRefs|SetBP_HomeBase-ref _returnvalue))
  ;[0 1 0.25] DEBUG
  (CallFunction|DebugPrint (Utilities|String|Append "BP Spawned/Ref Saved (" (Utilities|GetDisplayName _output_get) ")") "(R=0.058824,G=0.615686,B=0.192157,A=1.000000)" 2.0))

(event Custom|DebugPrint
  (params (DebugText :type String) (TextColor :type Linear%20Color%20Structure) (Duration :type Float%20%28double-precision%29) (DebugActor :type Actor%20Object%20Reference))
  ;[0 1 0.25] DEBUG
  (Development|PrintString (Utilities|String|Append "[" (Utilities|GetDisplayName DebugActor) "] " DebugText) (Utilities|Struct|BreakStruct_SaveGame (Variables|SaveGame|GetStruct_SaveGame)) true TextColor Duration))

(event Custom|SpawnClutter
  (bind _returnvalue (Math|Random|RandomFloatinRange 0.05 1.0))
  ;[0 1 0.7188] Spawn Clutter
  (Game|SpawnActorfromClass "/Game/Blueprints/BP_Clutter.BP_Clutter_C" (Math|Transform|MakeTransform (Math|Vector|MakeVector 0.0 (Math|Random|RandomFloatinRange -9.5e+03 9.5e+03) (Math|Random|RandomFloatinRange 2.5e+03 1e+04)) "0, 0, 0" (Math|Vector|MakeVector _returnvalue _returnvalue _returnvalue)) "AdjustIfPossibleButAlwaysSpawn" "OverrideRootScale" 0 0)
  (Math|Integer|IncrementInt (Variables|In-Game|GetClutterAmount)))