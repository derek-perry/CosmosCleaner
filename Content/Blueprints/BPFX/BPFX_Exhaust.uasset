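; BPFX_Exhaust is a short-lived exhaust effect actor that launches a mesh and fades it out.
; On BeginPlay it applies a velocity-change impulse opposite the actor's right vector, in Y and Z only, scaled by VelocityMultiplier.
; It creates a dynamic material instance, then a timeline lowers Opacity by a fixed step per update, making the fade frame-rate dependent.
; The actor destroys itself once Opacity is no longer positive.
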(event EventBeginPlay
  (bind _returnvalue (Transformation|GetActorRightVector))
  (bind _velocitymultiplier (Variables|Default|GetVelocityMultiplier))
  ;[0 1 0] BeginPlay
  ;[0.9688 0.9688 0.9688] Set Velocity
  (Physics|AddImpulse (Variables|Default|GetMesh_Exhaust) (Math|Vector|MakeVector 0.0 (* (* (.y _returnvalue) _velocitymultiplier) -1.0) (* (* (.z _returnvalue) _velocitymultiplier) -1.0)) "None" true)
  ;[0.9688 0.9688 0.9688] Setup Dynamic Material
  (Variables|Default|SetExhaustMat (Rendering|Material|GetMaterial (Variables|Default|GetMesh_Exhaust) 0))
  (bind _returnvalue_2 (Rendering|Material|CreateDynamicMaterialInstance (Variables|Default|GetMesh_Exhaust) 0 (Variables|Default|GetExhaustMat) "ExhaustMatDyn" :!class /Script/Engine.PrimitiveComponent))
  (Variables|Default|SetExhaustMatDyn _returnvalue_2)
  ;[0.9688 0.9688 0.9688] Fade Opacity
  (Timeline|ExhaustTimeline Play
    (:Update
      (Utilities|FlowControl|Sequence
        (:then_0
          (bind _returnvalue_3 (Rendering|Material|GetScalarParameterValue (Variables|Default|GetExhaustMatDyn) "Opacity" :!class /Script/Engine.MaterialInstanceDynamic))
          (Rendering|Material|SetScalarParameterValue (Variables|Default|GetExhaustMatDyn) "Opacity" (- _returnvalue_3 0.02) :!class /Script/Engine.MaterialInstanceDynamic))
        (:then_1
          (bind _returnvalue_4 (Rendering|Material|GetScalarParameterValue (Variables|Default|GetExhaustMatDyn) "Opacity" :!class /Script/Engine.MaterialInstanceDynamic))
          (if (not (> _returnvalue_4 0.0))
            (Actor|DestroyActor)))))))

(fn ConstructionScript)