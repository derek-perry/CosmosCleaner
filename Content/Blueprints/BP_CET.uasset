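; BP_CET is the player character, a thruster-driven body that starts at a fixed location with zeroed velocity and capsule rotation.
; Input axes drive physics impulses on the capsule: upward-only thrust along the actor's up vector and angular roll, both gated by and draining fuel.
; Holding Boost amplifies both and drains BoostAmnt, which is never checked here.
; Actions log through GameInstance_All's DebugPrint.
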(event EventBeginPlay
  ;[0 1 0] BeginPlay
  ;[0.9635 0.9635 0.9635] Reset Velocity
  (Variables|/Script/Engine.MovementComponent|SetVelocity (Variables|Character|GetCharacterMovement) "0, 0, 0")
  ;[0.9635 0.9635 0.9635] Reset Location
  (Transformation|SetActorLocation self "0.000000, 0,100.000000" false true)
  ;[0.9635 0.9635 0.9635] Reset Rotation
  (Transformation|SetWorldRotation (Variables|Collision|GetCapsuleComponent self) "0, 0, 0" false false)
  ;[0 1 0.25] DEBUG
  (bind _asgame_instance_all (Utilities|Casting|CastToGameInstance_All (Game|GetGameInstance)))
  (Default|DebugPrint _asgame_instance_all (Utilities|String|Append "Player Created (" (Utilities|GetDisplayName self) ")") "(R=0.058824,G=0.615686,B=0.192157,A=1.000000)" 2.0))

(fn ConstructionScript)

(event Input|ActionEvents|InputActionBoost
  (params (Key :type Key%20Structure :default "None"))
  ;[0 0 0] Press Boost to Boost
  (:Pressed
    ;[0.9583 0.9583 0.9583] Boost On
    (Variables|Movement|SetBoosting? true)
    ;[0 1 0.25] DEBUG
    (bind _asgame_instance_all (Utilities|Casting|CastToGameInstance_All (Game|GetGameInstance)))
    (Default|DebugPrint _asgame_instance_all "Boost On" "(R=0.058824,G=0.615686,B=0.192157,A=1.000000)" 2.0))
  (:Released
    ;[0.9583 0.9583 0.9583] Boost Off
    (Variables|Movement|SetBoosting? false)
    ;[0 1 0.25] DEBUG
    (bind _asgame_instance_all_2 (Utilities|Casting|CastToGameInstance_All (Game|GetGameInstance)))
    (Default|DebugPrint _asgame_instance_all_2 "Boost Off" "(R=0.058824,G=0.615686,B=0.192157,A=1.000000)" 2.0)))

(event Input|AxisEvents|InputAxisRollLeft/Right
  (params (AxisValue :type Float%20%28single-precision%29))
  (bind _returnvalue (Math|Float|Clamp(Float) AxisValue -1.0 1.0))
  ;[0 0 0] Press RollLeft/RollRight to Roll
  ;[0.9583 0.9583 0.9583] Able to Roll?
  (if (not (== _returnvalue 0.0))
    (if (> (Variables|Fuel|GetFuelAmnt) 0.0)
      (if (Variables|Movement|GetBoosting?)
        ;[1 0 0.2812] Roll (Boosted)
        (Class|PrimitiveComponent|AddAngularImpulseinDegrees (Variables|Collision|GetCapsuleComponent) (Math|Vector|MakeVector (* _returnvalue (Variables|Movement|GetTurnRate) (Variables|Movement|GetTurnRateBoosted) -1.0) 0.0 0.0) "None" false)
        ;[0 0.4141 1] Set Boost Amnt
        (Variables|Movement|SetBoostAmnt (- (Variables|Movement|GetBoostAmnt) (Variables|Movement|GetBoostRollLossMultiplier)))
        ;[0.4062 1 0] Set Fuel Amnt
        (Variables|Fuel|SetFuelAmnt (- (Variables|Fuel|GetFuelAmnt) (Variables|Fuel|GetFuelLossMultiplierLesser)))
        ;[0 1 0.25] DEBUG
        (bind _asgame_instance_all (Utilities|Casting|CastToGameInstance_All (Game|GetGameInstance)))
        (Default|DebugPrint _asgame_instance_all (Utilities|String|Append "RollLR-Boosted" " (" (Utilities|String|ToString(Float) _returnvalue) ")") "(R=0.058824,G=0.615686,B=0.192157,A=1.000000)" 1.0)
        (else
          ;[1 0 0.2812] Roll
          (Class|PrimitiveComponent|AddAngularImpulseinDegrees (Variables|Collision|GetCapsuleComponent) (Math|Vector|MakeVector (* _returnvalue (Variables|Movement|GetTurnRate) -1.0) 0.0 0.0) "None" false)
          ;[0.4062 1 0] Set Fuel Amnt
          (Variables|Fuel|SetFuelAmnt (- (Variables|Fuel|GetFuelAmnt) (Variables|Fuel|GetFuelLossMultiplierLesser)))
          ;[0 1 0.25] DEBUG
          (bind _asgame_instance_all_2 (Utilities|Casting|CastToGameInstance_All (Game|GetGameInstance)))
          (Default|DebugPrint _asgame_instance_all_2 (Utilities|String|Append "RollLR" " (" (Utilities|String|ToString(Float) _returnvalue) ")") "(R=0.058824,G=0.615686,B=0.192157,A=1.000000)" 1.0))))))

(event Input|AxisEvents|InputAxisThrustUp/Down
  (params (AxisValue :type Float%20%28single-precision%29))
  (bind _returnvalue (Math|Float|Clamp(Float) AxisValue 0.0))
  (bind _self self)
  (bind _self_2 self)
  (bind _thrustermultiplier (Variables|Movement|GetThrusterMultiplier))
  (bind _thrustermultiplier_2 (Variables|Movement|GetThrusterMultiplier))
  (bind _boostmultiplier (Variables|Movement|GetBoostMultiplier))
  (bind _fuellossmultiplier (Variables|Fuel|GetFuelLossMultiplier))
  (bind _returnvalue_2 (Transformation|GetActorUpVector _self_2))
  (bind _returnvalue_3 (Transformation|GetActorUpVector _self))
  (bind _returnvalue_4 (* _returnvalue _thrustermultiplier))
  (bind _returnvalue_5 (* _returnvalue _thrustermultiplier_2 _boostmultiplier))
  ;[0 0 0] Press Up/Down to Thrust
  ;[0.9531 0.9531 0.9531] Able to Thrust?
  (if (not (== _returnvalue 0.0))
    (if (> (Variables|Fuel|GetFuelAmnt) 0.0)
      (if (Variables|Movement|GetBoosting?)
        ;[1 0 0.2812] ThrustUD (Boosted)
        (Physics|AddImpulse (Variables|Collision|GetCapsuleComponent) (Math|Vector|MakeVector (* (.x _returnvalue_3) _returnvalue_5) (* (.y _returnvalue_3) _returnvalue_5) (* (.z _returnvalue_3) _returnvalue_5)) "None" false)
        ;[0 0.4141 1] Set Boost Amnt
        (Variables|Movement|SetBoostAmnt (- (Variables|Movement|GetBoostAmnt) (Variables|Movement|GetBoostUDLossMultiplier)))
        ;[0.4062 1 0] Set Fuel Amnt
        (Variables|Fuel|SetFuelAmnt (- (Variables|Fuel|GetFuelAmnt) (+ _fuellossmultiplier (* _fuellossmultiplier 0.36666))))
        ;[0 1 0.25] DEBUG
        (bind _asgame_instance_all (Utilities|Casting|CastToGameInstance_All (Game|GetGameInstance)))
        (Default|DebugPrint _asgame_instance_all (Utilities|String|Append "ThrustUD-Boosted" " (" (Utilities|String|ToString(Float) _returnvalue) ")") "(R=0.058824,G=0.615686,B=0.192157,A=1.000000)" 1.0)
        (else
          ;[1 0 0.2812] ThrustUD
          (Physics|AddImpulse (Variables|Collision|GetCapsuleComponent) (Math|Vector|MakeVector (* (.x _returnvalue_2) _returnvalue_4) (* (.y _returnvalue_2) _returnvalue_4) (* (.z _returnvalue_2) _returnvalue_4)) "None" false)
          ;[0.4062 1 0] Set Fuel Amnt
          (Variables|Fuel|SetFuelAmnt (- (Variables|Fuel|GetFuelAmnt) (Variables|Fuel|GetFuelLossMultiplier)))
          ;[0 1 0.25] DEBUG
          (bind _asgame_instance_all_2 (Utilities|Casting|CastToGameInstance_All (Game|GetGameInstance)))
          (Default|DebugPrint _asgame_instance_all_2 (Utilities|String|Append "ThrustUD" " (" (Utilities|String|ToString(Float) _returnvalue) ")") "(R=0.058824,G=0.615686,B=0.192157,A=1.000000)" 1.0))))))