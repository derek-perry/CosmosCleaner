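; Spawner actor that places a set number of clutter objects of a configured type at its own location when play begins.
; Each spawn is delegated to SpawnClutterSingle on the CosmosCleaner game instance with a random rotation on all three axes.
; The loop is recursive: the SpawnClutter event re-enters the count check after each spawn until the remaining count reaches zero, with no delay between spawns.
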(event Custom|SpawnClutter
  (bind _returnvalue (Math|Random|RandomFloatinRange -3.6e+02 3.6e+02))
  ;[0 1 0.7188] Spawn correct amount of Clutters
  (if (and (> (Variables|SpawnOptions|GetSpawnCount) 0) (> (Variables|SpawnOptions|GetSpawnCountRemaining) 0))
    (bind _ascosmos_cleaner_game_instance (Utilities|Casting|CastToCosmosCleaner_GameInstance (Game|GetGameInstance)))
    (Default|SpawnClutterSingle _ascosmos_cleaner_game_instance (Variables|SpawnOptions|GetSpawnType) (Math|Transform|MakeTransform (.location (Transformation|GetActorTransform)) (Math|Rotator|MakeRotator _returnvalue _returnvalue _returnvalue) "1.000000,1.000000,1.000000"))
    (Math|Integer|DecrementInt (Variables|SpawnOptions|GetSpawnCountRemaining)
      (:%20%20
        (CallFunction|SpawnClutter)))))

(event EventBeginPlay
  (bind _returnvalue (Math|Random|RandomFloatinRange -3.6e+02 3.6e+02))
  ;[0 1 0] Begin Play
  ;[0 1 0.7188] Spawn correct amount of Clutters
  (Variables|SpawnOptions|SetSpawnCountRemaining (Variables|SpawnOptions|GetSpawnCount))
  (if (and (> (Variables|SpawnOptions|GetSpawnCount) 0) (> (Variables|SpawnOptions|GetSpawnCountRemaining) 0))
    (bind _ascosmos_cleaner_game_instance (Utilities|Casting|CastToCosmosCleaner_GameInstance (Game|GetGameInstance)))
    (Default|SpawnClutterSingle _ascosmos_cleaner_game_instance (Variables|SpawnOptions|GetSpawnType) (Math|Transform|MakeTransform (.location (Transformation|GetActorTransform)) (Math|Rotator|MakeRotator _returnvalue _returnvalue _returnvalue) "1.000000,1.000000,1.000000"))
    (Math|Integer|DecrementInt (Variables|SpawnOptions|GetSpawnCountRemaining)
      (:%20%20
        (CallFunction|SpawnClutter)))))

(fn ConstructionScript)