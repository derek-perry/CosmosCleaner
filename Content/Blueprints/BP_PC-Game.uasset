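; In-game player controller for Cosmos Cleaner that opens the pause and dashboard menus from input or custom events.
; Pause closes an open settings menu, or creates W_Pause when no home or dashboard widget exists, stopping the character's boost and collecting.
; The dashboard action opens the homebase widget when the player is inside the home base, otherwise the dashboard.
; Widget references on the game instance serve as guards against stacking menus.
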(event Custom|PressCargo
  ;[0 0 0] Press Dashboard Button
  ;[0.974 0.974 0.974] Existing W_Pause?
  (Utilities|IsValid (Variables|Default|GetW_Pause)
    (:Is%20Not%20Valid
      ;[0.974 0.974 0.974] Existing W_Settings?
      (bind _ascosmos_cleaner_game_instance (Utilities|Casting|CastToCosmosCleaner_GameInstance (Game|GetGameInstance))
        (:then
          (Utilities|IsValid (Variables|/Game/Blueprints/CosmosCleaner_GameInstance.CosmosCleaner_GameInstance_C|GetW_Settings _ascosmos_cleaner_game_instance)
            (:Is%20Not%20Valid
              ;[0.9896 0.9896 0.9896] Check if Player is Inside Homebase Area
              (Utilities|IsValid (Variables|/Game/Blueprints/CosmosCleaner_GameInstance.CosmosCleaner_GameInstance_C|GetBP_HomeBase-ref _ascosmos_cleaner_game_instance)
                (:Is%20Valid
                  (if (Variables|/Game/Blueprints/BP_HomeBase.BP_HomeBase_C|GetPlayerInside? (Variables|/Game/Blueprints/CosmosCleaner_GameInstance.CosmosCleaner_GameInstance_C|GetBP_HomeBase-ref _ascosmos_cleaner_game_instance))
                    ;[0.974 0.974 0.974] Existing W_Home?
                    (Utilities|IsValid (Variables|/Game/Blueprints/CosmosCleaner_GameInstance.CosmosCleaner_GameInstance_C|GetW_Home _ascosmos_cleaner_game_instance)
                      (:Is%20Valid
                        _)
                      (:Is%20Not%20Valid
                        ;[0.8542 0.5278 0.3337] Create Widget - W_Homebase
                        (Default|WidgetCreateHomebase _ascosmos_cleaner_game_instance :!label _label)))
                    ;[0.25 0 1] Play Sound : Click
                    (Audio|PlaySound2D "/Game/Audio/SFX/A_Cue_SFX_Click.A_Cue_SFX_Click" 1.0 1.0 0.0 0 0)
                    (else
                      ;[0.974 0.974 0.974] Existing W_Dashboard?
                      (Utilities|IsValid (Variables|/Game/Blueprints/CosmosCleaner_GameInstance.CosmosCleaner_GameInstance_C|GetW_Dashboard _ascosmos_cleaner_game_instance)
                        (:Is%20Valid
                          _)
                        (:Is%20Not%20Valid
                          ;[0.8542 0.5278 0.3337] Create Widget - W_Dashboard
                          (Default|WidgetCreateDashboard _ascosmos_cleaner_game_instance)))
                      ;[0.25 0 1] Play Sound : Click
                      (Audio|PlaySound2D "/Game/Audio/SFX/A_Cue_SFX_Click.A_Cue_SFX_Click" 1.0 1.0 0.0 0 0))))))))
        (:CastFailed
          (goto _label))))))

(event Custom|PressPause
  ;[0 0 0] Press Pause Button
  ;[0.974 0.974 0.974] Existing W_Pause?
  (Utilities|IsValid (Variables|Default|GetW_Pause)
    (:Is%20Not%20Valid
      ;[0.974 0.974 0.974] Existing W_Settings?
      (bind _ascosmos_cleaner_game_instance (Utilities|Casting|CastToCosmosCleaner_GameInstance (Game|GetGameInstance))
        (:then
          (Utilities|IsValid (Variables|/Game/Blueprints/CosmosCleaner_GameInstance.CosmosCleaner_GameInstance_C|GetW_Settings _ascosmos_cleaner_game_instance)
            (:Is%20Valid
              ;[0.9688 0.9688 0.9688] Check for Open Settings Menu
              (if (Variables|/Game/Widgets/W_Menu-Settings.W_Menu-Settings_C|GetMenuOpen? (Variables|/Game/Blueprints/CosmosCleaner_GameInstance.CosmosCleaner_GameInstance_C|GetW_Settings _ascosmos_cleaner_game_instance))
                (Default|MenuHideAll (Variables|/Game/Blueprints/CosmosCleaner_GameInstance.CosmosCleaner_GameInstance_C|GetW_Settings _ascosmos_cleaner_game_instance))
                ;[0.25 0 1] Play Sound : Click
                (Audio|PlaySound2D "/Game/Audio/SFX/A_Cue_SFX_Click.A_Cue_SFX_Click" 1.0 1.0 0.0 0 0)))
            (:Is%20Not%20Valid
              ;[0.974 0.974 0.974] Existing W_Home?
              (Utilities|IsValid (Variables|/Game/Blueprints/CosmosCleaner_GameInstance.CosmosCleaner_GameInstance_C|GetW_Home _ascosmos_cleaner_game_instance)
                (:Is%20Not%20Valid
                  ;[0.974 0.974 0.974] Existing W_Dashboard?
                  (Utilities|IsValid (Variables|/Game/Blueprints/CosmosCleaner_GameInstance.CosmosCleaner_GameInstance_C|GetW_Dashboard _ascosmos_cleaner_game_instance)
                    (:Is%20Not%20Valid
                      ;[0.25 0 1] Play Sound : Click
                      (Audio|PlaySound2D "/Game/Audio/SFX/A_Cue_SFX_Click.A_Cue_SFX_Click" 1.0 1.0 0.0 0 0 :!label _label)
                      ;[0.8542 0.5278 0.3337] Create Widget - W_Pause
                      (bind _returnvalue (UserInterface|CreateWidget "/Game/Widgets/W_Pause.W_Pause_C"))
                      (bind _output_get (Variables|Default|SetW_Pause _returnvalue))
                      (UserInterface|Viewport|AddtoViewport _output_get 0)
                      (bind _ascosmos_cleaner_game_instance_2 (Utilities|Casting|CastToCosmosCleaner_GameInstance (Game|GetGameInstance)))
                      (Variables|/Game/Blueprints/BP_Character/BP_Character.BP_Character_C|SetBoosting? (Variables|/Game/Blueprints/CosmosCleaner_GameInstance.CosmosCleaner_GameInstance_C|GetBP_Character-ref _ascosmos_cleaner_game_instance_2) false)
                      (Default|BoostRegenStart (Variables|/Game/Blueprints/CosmosCleaner_GameInstance.CosmosCleaner_GameInstance_C|GetBP_Character-ref _ascosmos_cleaner_game_instance_2))
                      (Default|CollectingStop (Variables|/Game/Blueprints/CosmosCleaner_GameInstance.CosmosCleaner_GameInstance_C|GetBP_Character-ref _ascosmos_cleaner_game_instance_2))
                      ;[0 1 0.25] DEBUG
                      (Default|DebugPrint _ascosmos_cleaner_game_instance_2 (Utilities|String|Append "Widget Created (" (Utilities|GetDisplayName _output_get) ")") "(R=0.058824,G=0.615686,B=0.192157,A=1.000000)" 2.0 0 "None"))))))))
        (:CastFailed
          (goto _label))))))

(event Input|EnhancedActionEvents|EnhancedInputActionIA_Pause
  (params (ActionValue :type Boolean) (ElapsedSeconds :type Float%20%28double-precision%29) (TriggeredSeconds :type Float%20%28double-precision%29) (InputAction :type Input%20Action%20Object%20Reference :default "/Game/Input/IA_Pause.IA_Pause"))
  ;[0 0 0] Press Pause Button
  (:Started
    ;[0.974 0.974 0.974] Existing W_Pause?
    (Utilities|IsValid (Variables|Default|GetW_Pause)
      (:Is%20Not%20Valid
        ;[0.974 0.974 0.974] Existing W_Settings?
        (bind _ascosmos_cleaner_game_instance (Utilities|Casting|CastToCosmosCleaner_GameInstance (Game|GetGameInstance))
          (:then
            (Utilities|IsValid (Variables|/Game/Blueprints/CosmosCleaner_GameInstance.CosmosCleaner_GameInstance_C|GetW_Settings _ascosmos_cleaner_game_instance)
              (:Is%20Valid
                ;[0.9688 0.9688 0.9688] Check for Open Settings Menu
                (if (Variables|/Game/Widgets/W_Menu-Settings.W_Menu-Settings_C|GetMenuOpen? (Variables|/Game/Blueprints/CosmosCleaner_GameInstance.CosmosCleaner_GameInstance_C|GetW_Settings _ascosmos_cleaner_game_instance))
                  (Default|MenuHideAll (Variables|/Game/Blueprints/CosmosCleaner_GameInstance.CosmosCleaner_GameInstance_C|GetW_Settings _ascosmos_cleaner_game_instance))
                  ;[0.25 0 1] Play Sound : Click
                  (Audio|PlaySound2D "/Game/Audio/SFX/A_Cue_SFX_Click.A_Cue_SFX_Click" 1.0 1.0 0.0 0 0)))
              (:Is%20Not%20Valid
                ;[0.974 0.974 0.974] Existing W_Home?
                (Utilities|IsValid (Variables|/Game/Blueprints/CosmosCleaner_GameInstance.CosmosCleaner_GameInstance_C|GetW_Home _ascosmos_cleaner_game_instance)
                  (:Is%20Not%20Valid
                    ;[0.974 0.974 0.974] Existing W_Dashboard?
                    (Utilities|IsValid (Variables|/Game/Blueprints/CosmosCleaner_GameInstance.CosmosCleaner_GameInstance_C|GetW_Dashboard _ascosmos_cleaner_game_instance)
                      (:Is%20Not%20Valid
                        ;[0.25 0 1] Play Sound : Click
                        (Audio|PlaySound2D "/Game/Audio/SFX/A_Cue_SFX_Click.A_Cue_SFX_Click" 1.0 1.0 0.0 0 0 :!label _label)
                        ;[0.8542 0.5278 0.3337] Create Widget - W_Pause
                        (bind _returnvalue (UserInterface|CreateWidget "/Game/Widgets/W_Pause.W_Pause_C"))
                        (bind _output_get (Variables|Default|SetW_Pause _returnvalue))
                        (UserInterface|Viewport|AddtoViewport _output_get 0)
                        (bind _ascosmos_cleaner_game_instance_2 (Utilities|Casting|CastToCosmosCleaner_GameInstance (Game|GetGameInstance)))
                        (Variables|/Game/Blueprints/BP_Character/BP_Character.BP_Character_C|SetBoosting? (Variables|/Game/Blueprints/CosmosCleaner_GameInstance.CosmosCleaner_GameInstance_C|GetBP_Character-ref _ascosmos_cleaner_game_instance_2) false)
                        (Default|BoostRegenStart (Variables|/Game/Blueprints/CosmosCleaner_GameInstance.CosmosCleaner_GameInstance_C|GetBP_Character-ref _ascosmos_cleaner_game_instance_2))
                        (Default|CollectingStop (Variables|/Game/Blueprints/CosmosCleaner_GameInstance.CosmosCleaner_GameInstance_C|GetBP_Character-ref _ascosmos_cleaner_game_instance_2))
                        ;[0 1 0.25] DEBUG
                        (Default|DebugPrint _ascosmos_cleaner_game_instance_2 (Utilities|String|Append "Widget Created (" (Utilities|GetDisplayName _output_get) ")") "(R=0.058824,G=0.615686,B=0.192157,A=1.000000)" 2.0 0 "None"))))))))
          (:CastFailed
            (goto _label)))))))

(event Input|EnhancedActionEvents|EnhancedInputActionIA_Dashboard
  (params (ActionValue :type Boolean) (ElapsedSeconds :type Float%20%28double-precision%29) (TriggeredSeconds :type Float%20%28double-precision%29) (InputAction :type Input%20Action%20Object%20Reference :default "/Game/Input/IA_Dashboard.IA_Dashboard"))
  ;[0 0 0] Press Dashboard Button
  (:Started
    ;[0.974 0.974 0.974] Existing W_Pause?
    (Utilities|IsValid (Variables|Default|GetW_Pause)
      (:Is%20Not%20Valid
        ;[0.974 0.974 0.974] Existing W_Settings?
        (bind _ascosmos_cleaner_game_instance (Utilities|Casting|CastToCosmosCleaner_GameInstance (Game|GetGameInstance))
          (:then
            (Utilities|IsValid (Variables|/Game/Blueprints/CosmosCleaner_GameInstance.CosmosCleaner_GameInstance_C|GetW_Settings _ascosmos_cleaner_game_instance)
              (:Is%20Not%20Valid
                ;[0.9896 0.9896 0.9896] Check if Player is Inside Homebase Area
                (Utilities|IsValid (Variables|/Game/Blueprints/CosmosCleaner_GameInstance.CosmosCleaner_GameInstance_C|GetBP_HomeBase-ref _ascosmos_cleaner_game_instance)
                  (:Is%20Valid
                    (if (Variables|/Game/Blueprints/BP_HomeBase.BP_HomeBase_C|GetPlayerInside? (Variables|/Game/Blueprints/CosmosCleaner_GameInstance.CosmosCleaner_GameInstance_C|GetBP_HomeBase-ref _ascosmos_cleaner_game_instance))
                      ;[0.974 0.974 0.974] Existing W_Home?
                      (Utilities|IsValid (Variables|/Game/Blueprints/CosmosCleaner_GameInstance.CosmosCleaner_GameInstance_C|GetW_Home _ascosmos_cleaner_game_instance)
                        (:Is%20Valid
                          _)
                        (:Is%20Not%20Valid
                          ;[0.8542 0.5278 0.3337] Create Widget - W_Homebase
                          (Default|WidgetCreateHomebase _ascosmos_cleaner_game_instance :!label _label)))
                      ;[0.25 0 1] Play Sound : Click
                      (Audio|PlaySound2D "/Game/Audio/SFX/A_Cue_SFX_Click.A_Cue_SFX_Click" 1.0 1.0 0.0 0 0)
                      (else
                        ;[0.974 0.974 0.974] Existing W_Dashboard?
                        (Utilities|IsValid (Variables|/Game/Blueprints/CosmosCleaner_GameInstance.CosmosCleaner_GameInstance_C|GetW_Dashboard _ascosmos_cleaner_game_instance)
                          (:Is%20Valid
                            _)
                          (:Is%20Not%20Valid
                            ;[0.8542 0.5278 0.3337] Create Widget - W_Dashboard
                            (Default|WidgetCreateDashboard _ascosmos_cleaner_game_instance)))
                        ;[0.25 0 1] Play Sound : Click
                        (Audio|PlaySound2D "/Game/Audio/SFX/A_Cue_SFX_Click.A_Cue_SFX_Click" 1.0 1.0 0.0 0 0))))))))
          (:CastFailed
            (goto _label)))))))

(fn ConstructionScript)