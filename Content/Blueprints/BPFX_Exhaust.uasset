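; BPFX_Exhaust is a short-lived exhaust effect actor that launches a mesh and fades it out.
; On BeginPlay it pushes ExhaustMesh opposite the BP_CET player character's right vector, using only Y and Z, scaled by VelocityMultiplier.
; A timeline lowers the Opacity of a dynamic material instance by a fixed step per update, making the fade frame-rate dependent, and destroys the actor at zero.
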(event EventBeginPlay
  (bind _velocitymultiplier (Variables|Default|GetVelocityMultiplier))
  ;[0 1 0] BeginPlay
  ;[0 1 0.7188] Save Ref of BP_CET
  (bind _asbp_cet (Utilities|Casting|CastToBP_CET (Game|GetPlayerCharacter 0)))
  (Variables|Default|SetBP_CET-ref _asbp_cet)
  ;[0.9688 0.9688 0.9688] Set Velocity
  (Physics|AddImpulse (Variables|Default|GetExhaustMesh) (Math|Vector|MakeVector 0.0 (* (* (.y (Transformation|GetActorRightVector _asbp_cet)) _velocitymultiplier) -1.0) (* (* (.z (Transformation|GetActorRightVector _asbp_cet)) _velocitymultiplier) -1.0)) "None" true)
  ;[0.9688 0.9688 0.9688] Setup Dynamic Material
  (Variables|Default|SetExhaustMat (Rendering|Material|GetMaterial (Variables|Default|GetExhaustMesh) 0))
  (bind _returnvalue (Rendering|Material|CreateDynamicMaterialInstance (Variables|Default|GetExhaustMesh) 0 (Variables|Default|GetExhaustMat) "ExhaustMatDyn" :!class /Script/Engine.PrimitiveComponent))
  (Variables|Default|SetExhaustMatDyn _returnvalue)
  ;[0.9688 0.9688 0.9688] Fade Opacity
  (Timeline|ExhaustTimeline Play
    (:Update
      (Utilities|FlowControl|Sequence
        (:then_0
          (bind _returnvalue_2 (Rendering|Material|GetScalarParameterValue (Variables|Default|GetExhaustMatDyn) "Opacity" :!class /Script/Engine.MaterialInstanceDynamic))
          (Rendering|Material|SetScalarParameterValue (Variables|Default|GetExhaustMatDyn) "Opacity" (- _returnvalue_2 0.02) :!class /Script/Engine.MaterialInstanceDynamic))
        (:then_1
          (bind _returnvalue_3 (Rendering|Material|GetScalarParameterValue (Variables|Default|GetExhaustMatDyn) "Opacity" :!class /Script/Engine.MaterialInstanceDynamic))
          (if (not (> _returnvalue_3 0.0))
            (Actor|DestroyActor)))))))

(fn ConstructionScript)