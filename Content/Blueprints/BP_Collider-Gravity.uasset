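; BP_Collider-Gravity is a trigger volume that defines a zone where the player character is subject to gravity.
; When a BP_Character enters its box collision, gravity is enabled on that character's capsule component, and leaving the box disables it again.
; Both events also send a debug message through CosmosCleaner_GameInstance's DebugPrint to report the gravity state.
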(event OnComponentBeginOverlap(BoxCollision)
  (params (OverlappedComponent :type Primitive%20Component%20Object%20Reference) (OtherActor :type Actor%20Object%20Reference) (OtherComp :type Primitive%20Component%20Object%20Reference) (OtherBodyIndex :type Integer) (bFromSweep :type Boolean) (SweepResult :type Hit%20Result%20Structure%20%28by%20ref%29))
  ;[0.9427 0.9427 0.9427] Collider Check - Gravity
  (bind _asbp_character (Utilities|Casting|CastToBP_Character OtherActor))
  (Physics|SetEnableGravity (Variables|/Script/Engine.Character|GetCapsuleComponent _asbp_character) true)
  ;[0 1 0.25] DEBUG
  (bind _asgame_instance_all (Utilities|Casting|CastToCosmosCleaner_GameInstance (Game|GetGameInstance)))
  (Default|DebugPrint _asgame_instance_all "Gravity = -98.0" "(R=0.058824,G=0.615686,B=0.192157,A=1.000000)" 2.0 self "None"))

(event OnComponentEndOverlap(BoxCollision)
  (params (OverlappedComponent :type Primitive%20Component%20Object%20Reference) (OtherActor :type Actor%20Object%20Reference) (OtherComp :type Primitive%20Component%20Object%20Reference) (OtherBodyIndex :type Integer))
  ;[0.9427 0.9427 0.9427] Collider Check - Gravity
  (bind _asbp_character (Utilities|Casting|CastToBP_Character OtherActor))
  (Physics|SetEnableGravity (Variables|/Script/Engine.Character|GetCapsuleComponent _asbp_character) false)
  ;[0 1 0.25] DEBUG
  (bind _asgame_instance_all (Utilities|Casting|CastToCosmosCleaner_GameInstance (Game|GetGameInstance)))
  (Default|DebugPrint _asgame_instance_all "Gravity = 0" "(R=0.058824,G=0.615686,B=0.192157,A=1.000000)" 2.0 self "None"))

(fn ConstructionScript)