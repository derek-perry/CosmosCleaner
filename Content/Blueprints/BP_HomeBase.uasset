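; BP_HomeBase is a home base actor that opens the home base widget when a BP_CET enters its box collider.
; On begin overlap, it casts the actor to BP_CET and its controller to BP_PC, then calls CreateWidgetHomeBase on that controller.
; Entering and exiting send debug prints through GameInstance_All; exit does not remove the widget.
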(event OnComponentBeginOverlap(BoxCollision_HomeBase)
  (params (OverlappedComponent :type Primitive%20Component%20Object%20Reference) (OtherActor :type Actor%20Object%20Reference) (OtherComp :type Primitive%20Component%20Object%20Reference) (OtherBodyIndex :type Integer) (bFromSweep :type Boolean) (SweepResult :type Hit%20Result%20Structure%20%28by%20ref%29))
  ;[0.9583 0.9583 0.9583] Collider Check - HomeBase
  (bind _asbp_cet (Utilities|Casting|CastToBP_CET OtherActor))
  (bind _asbp_pc (Utilities|Casting|CastToBP_PC (Pawn|GetController _asbp_cet)))
  (Default|CreateWidgetHomeBase _asbp_pc)
  ;[0 1 0.25] DEBUG
  (bind _asgame_instance_all (Utilities|Casting|CastToGameInstance_All (Game|GetGameInstance)))
  (Default|DebugPrint _asgame_instance_all "HomeBase Entered" "(R=0.058824,G=0.615686,B=0.192157,A=1.000000)" 2.0 self))

(event OnComponentEndOverlap(BoxCollision_HomeBase)
  (params (OverlappedComponent :type Primitive%20Component%20Object%20Reference) (OtherActor :type Actor%20Object%20Reference) (OtherComp :type Primitive%20Component%20Object%20Reference) (OtherBodyIndex :type Integer))
  ;[0.9583 0.9583 0.9583] Collider Check - HomeBase
  ;[0 1 0.25] DEBUG
  (bind _asgame_instance_all (Utilities|Casting|CastToGameInstance_All (Game|GetGameInstance)))
  (Default|DebugPrint _asgame_instance_all "HomeBase Exited" "(R=0.058824,G=0.615686,B=0.192157,A=1.000000)" 2.0 self))

(fn ConstructionScript)